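; Test Blueprint for a physics-driven, player-steered mesh, apparently a bowling ball.
; Forward/back input applies a mass-independent force along the Forward spring arm's heading, rotated by the negated mesh rotation, with HitHeight adding forward bias in either direction.
; Right/left input applies yaw torque to the mesh, turns the spring arm and re-aims the camera from its target rotation with a downward pitch.
; An unconnected pitch-torque node never runs.
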(event EventMoveRightAxis
  (params (Axis :type Float%20%28single-precision%29))
  (bind _camera (Variables|Components|GetCamera))
  (bind _forward (Variables|Components|GetForward))
  (Class|PrimitiveComponent|AddTorqueinDegrees (Variables|Components|GetMesh) (Math|Vector|MakeVector 0.0 0.0 (* Axis (Variables|Movement|GetTorque))) "None" true)
  (Transformation|AddLocalRotation _forward (Math|Rotator|MakeRotator 0.0 0.0 (* Axis (Variables|Movement|GetSpinRate))) false false)
  (Transformation|SetRelativeRotation _camera (Class|SpringArmComponent|GetTargetRotation _forward) false false)
  (Transformation|AddLocalRotation _camera "-30.000000, 0, 0" false false))

(event EventMoveForwardAxis
  (params (Axis :type Float%20%28single-precision%29))
  (bind _mesh (Variables|Components|GetMesh))
  (bind _forward (Variables|Components|GetForward))
  (Physics|AddForce _mesh (Math|Vector|RotateVector (+ (* (Math|Vector|GetForwardVector _forward) (* Axis (Variables|Movement|GetHitForce))) (* (* (Math|Vector|GetForwardVector _forward) (Variables|Movement|GetHitHeight)) (Math|Float|Absolute(Float) Axis))) (Class|KismetMathLibrary|NegateRotator (Variables|/Script/Engine.SceneComponent|GetRelativeRotation _mesh))) "None" true))