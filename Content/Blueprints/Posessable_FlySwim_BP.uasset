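; Possessable physics pawn that glides at a set height while possessed and falls under gravity when released.
; Possession disables gravity and moves the mesh to a fixed Z; Jump adds a forward swim impulse, and Turn yaws the controller.
; While possessed, each tick clamps horizontal speed and uses a downward trace to offset the mesh toward MaxHeight above the surface below.
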(event EventBeginPlay
  (|CallParentFunction)
  (Physics|SetEnableGravity (Variables|Default|GetStaticMesh) true)
  (Variables|Default|Setposs false))

(event Collision|EventActorBeginOverlap
  (params (OtherActor :type Actor%20Object%20Reference))
  (|CallParentFunction OtherActor) ; This node is disabled and will not be called.\nDrag off pins to build functionality.
)

(event EventTick
  (params (DeltaSeconds :type Float%20%28single-precision%29))
  (|CallParentFunction DeltaSeconds)
  (CallFunction|LimitVelocity (Variables|Default|GetMax_Velocity)))

(event EventPossessed
  (params (NewController :type Controller%20Object%20Reference))
  (bind _staticmesh (Variables|Default|GetStaticMesh))
  (bind _returnvalue (Transformation|GetWorldLocation _staticmesh))
  (Variables|Default|Setposs true)
  (Physics|SetEnableGravity _staticmesh false)
  (Transformation|SetWorldLocation _staticmesh (Math|Vector|MakeVector (.x _returnvalue) (.y _returnvalue) 3e+02) true true))

(event EventUnpossessed
  (params (OldController :type Controller%20Object%20Reference))
  (Variables|Default|Setposs false)
  (Physics|SetEnableGravity (Variables|Default|GetStaticMesh) true))

(event Input|ActionEvents|InputActionJump
  (params (Key :type Key%20Structure :default "None"))
  (:Pressed
    (CallFunction|Swim (Variables|Default|GetSwim_speed))))

(event Input|AxisEvents|InputAxisTurn
  (params (AxisValue :type Float%20%28single-precision%29))
  ;[1 1 1] Turn's the current pawn based on camera
  (Pawn|Input|AddControllerYawInput AxisValue))

(fn ConstructionScript
  (Variables|Default|SetPossessableComponent (Variables|Default|GetPosessable_FS_component_BP))
  (|CallParentFunction))

(fn Swim
  (params (Swim_speed :type Float%20%28single-precision%29))
  ;[1 1 1] Forward motion
  (Physics|AddImpulse (Variables|Default|GetStaticMesh) (* (Math|Vector|GetForwardVector (Variables|Default|GetForward)) Swim_speed) "None" true))

(fn LimitVelocity
  (params (MaxVel :type Float%20%28single-precision%29))
  (bind _returnvalue (Transformation|GetVelocity))
  (bind _staticmesh (Variables|Default|GetStaticMesh))
  (bind _returnvalue_2 (Math|Vector|MakeVector (.x _returnvalue) (.y _returnvalue) 0.0))
  (bind _returnvalue_3 (Transformation|GetWorldLocation _staticmesh))
  (bind _returnvalue_4 (Math|Vector|ClampVectorSize _returnvalue_2 0.0 MaxVel))
  (if (Variables|Default|Getposs)
    (if (> (Math|Vector|VectorLength _returnvalue_2) MaxVel)
      (Physics|SetPhysicsLinearVelocity (Variables|Default|GetStaticMesh) (Math|Vector|MakeVector (.x _returnvalue_4) (.y _returnvalue_4) (.z _returnvalue)) false "None"))
    ;[1 1 1] This mess handles height above object
    (bind _outhit (Collision|LineTraceByChannel _returnvalue_3 (+ _returnvalue_3 (* (* (Math|Vector|GetUpVector _staticmesh) -1.0) 1.5e+03)) "TraceTypeQuery1" false 0 "None"))
    (Transformation|AddWorldOffset (Variables|Default|GetStaticMesh) (Math|Vector|MakeVector 0.0 0.0 (- (Variables|Default|GetMax_height) (.Distance (Collision|BreakHitResult _outhit)))) true true)))