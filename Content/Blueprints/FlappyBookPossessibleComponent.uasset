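; Possessable-pawn component that drives a flappy book prop the player hops, glides, steers and scares with.
; Movement button applies a physics jump impulse; holding Scare glides with raised damping and forward impulses, releasing it scares with a short cooldown.
; Triggers strafe on release or turn the pawn when held.
; Tick traces down to land and freeze physics, and up to apply a stamina hit on overhead contact.
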(event EventBeginPlay)

(event EventTick
  (params (DeltaSeconds :type Float%20%28single-precision%29))
  (|LineTraceCollideLogic)
  (if (Variables|Default|GetmIsGliding)
    (|GlidingFowardMovement))
  (bind _deltatimeout (|TurnLeftLogic DeltaSeconds))
  (|TurnRightLogic _deltatimeout)
  (|ScarlingJumpCooldownTimer _deltatimeout))

(fn GetStaticMesh
  (bind _aspossessable_pawn (Utilities|Casting|CastToPossessablePawn (Components|GetOwner)))
  (return (Variables|/Script/SummerDeliverables.PossessablePawn|GetStaticMeshComponent _aspossessable_pawn)))

(fn GetSkeletalMesh
  (bind _aspossessable_pawn (Utilities|Casting|CastToPossessablePawn (Components|GetOwner)))
  (return (Variables|/Script/SummerDeliverables.PossessablePawn|GetSkeletalMeshComponent _aspossessable_pawn)))

(event EventRightTrigger
  (return))

(event EventRightTriggerRelease
  (|Outputs) ; enters at Released
)

(event EventLeftTrigger
  (return))

(event EventLeftTriggerRelease
  (|Outputs) ; enters at Released
)

(event EventScareButton
  (return))

(event EventScareButtonRelease
  (|Outputs) ; enters at Released
)

(event EventMoveForwardAxis
  (params (Axis :type Float%20%28single-precision%29)))

(event EventMoveRightAxis
  (params (Axis :type Float%20%28single-precision%29)))

(event EventMoveButton
  (return))

(event EventMoveButtonRelease
  (|Outputs) ; enters at Released
)