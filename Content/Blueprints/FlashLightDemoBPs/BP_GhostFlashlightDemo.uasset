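; Demo ghost enemy for flashlight testing that drifts forward until an overlap marks it as hit.
; While hit it stops advancing, loses health over TimeTilDeath and shakes its skeletal mesh by alternating random offsets and resets.
; Any overlap starts damage, but ending it requires the other actor's "None" tag.
; On death it moves to the Spawner's location and stops updating, with debug prints reporting health and death.
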(event Custom|Death
  (Transformation|SetWorldLocation (Variables|Default|GetStaticMesh) (+ (Transformation|GetActorLocation (Variables|Default|GetSpawner)) "0, 0, 0") false false)
  (Transformation|SetRelativeLocation (Variables|Default|GetSkeletalMesh) "0, 0, 0" false true)
  (Variables|Default|SetbHasDied true)
  (Development|PrintString "died"))

(event EventBeginPlay
  (Variables|Default|SetbBeingHit false)
  (Variables|Default|SetbHasDied false))

(event EventTick
  (params (DeltaSeconds :type Float%20%28single-precision%29))
  (bind _skeletalmesh (Variables|Default|GetSkeletalMesh))
  (if (not (Variables|Default|GetbHasDied))
    (if (Variables|Default|GetbBeingHit)
      (bind _output_get (Variables|Default|SetHealth (+ (Variables|Default|GetHealth) (* (* DeltaSeconds (/ 1e+02 (Variables|Default|GetTimeTilDeath))) -1.0))))
      (Development|PrintString (Utilities|String|Append "Ghosty taking damage; Health = " (Utilities|String|ToString(Float) _output_get)))
      (Utilities|FlowControl|FlipFlop
        (:A
          (Transformation|AddWorldOffset _skeletalmesh (* (Math|Random|RandomUnitVector) (Variables|Default|GetShake-ness)) false true))
        (:B
          (Transformation|SetRelativeLocation _skeletalmesh "0, 0, 0" false true)))
      (if (< _output_get 0.0)
        (CallFunction|Death))
      (else
        (Transformation|AddLocalOffset (Variables|Default|GetStaticMesh) (* "1.000000, 0, 0" (* DeltaSeconds (Variables|Default|GetSpeed))) false false)))))

(event Collision|EventActorBeginOverlap
  (params (OtherActor :type Actor%20Object%20Reference))
  (Variables|Default|SetbBeingHit true))

(event Collision|EventActorEndOverlap
  (params (OtherActor :type Actor%20Object%20Reference))
  (if (Utilities|Array|ContainsItem (Variables|/Script/Engine.Actor|GetTags OtherActor) "")
    (Variables|Default|SetbBeingHit false)))

(fn ConstructionScript)

(fn MoveForward
  (Transformation|AddActorLocalOffset "1.000000, 0, 0" false false))