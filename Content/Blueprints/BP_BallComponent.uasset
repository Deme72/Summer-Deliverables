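; Possessable component on BP_Ball that lets the player steer a ball fired from a launcher.
; LaunchingBall stores the launcher and steering strength, then applies a power-scaled force.
; Right-axis input spins the ball, turns the spring arm camera and bends velocity toward camera forward while preserving speed.
; Bounce calls Eject past a bounce limit, while EndInteract returns control to the launcher and destroys the ball.
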(event EventBeginPlay
  ;[1 1 1] Gets a reference the ball we are currently possessing
  (bind _asbp_ball (Utilities|Casting|CastToBP_Ball (Components|GetOwner self)))
  (Variables|Default|SetBall_ref _asbp_ball))

(event EventTick
  (params (DeltaSeconds :type Float%20%28single-precision%29)))

(event EventEndInteract
  (bind _asbp_ball_launcher_component (Utilities|Casting|CastToBP_BallLauncherComponent (Variables|/Script/SummerDeliverables.PossessablePawn|GetPossessableComponent (Variables|Default|GetLauncher_ref))))
  (Variables|/Game/Blueprints/BP_BallLauncherComponent.BP_BallLauncherComponent_C|SetControling _asbp_ball_launcher_component true)
  (Actor|DestroyActor (Variables|Default|GetBall_ref)))

(event EventMoveRightAxis
  (params (Axis :type Float%20%28single-precision%29))
  (bind _ball_ref (Variables|Default|GetBall_ref))
  (bind _springarm (Variables|/Game/Blueprints/BP_Ball.BP_Ball_C|GetSpringArm _ball_ref))
  (bind _staticmeshcomponent (Variables|/Script/SummerDeliverables.PossessablePawn|GetStaticMeshComponent _ball_ref))
  (bind _staticmeshcomponent_2 (Variables|/Script/SummerDeliverables.PossessablePawn|GetStaticMeshComponent _ball_ref))
  (bind _camera (Variables|/Game/Blueprints/BP_Ball.BP_Ball_C|GetCamera _ball_ref))
  (bind _movement_refernce (Variables|/Game/Blueprints/BP_Ball.BP_Ball_C|GetMovement%20Refernce _ball_ref))
  (bind _returnvalue (Transformation|GetComponentVelocity _staticmeshcomponent))
  (bind _returnvalue_2 (Math|Vector|GetForwardVector _camera))
  (bind (_x _y _z) (Math|Vector|BreakVector _returnvalue))
  (bind (_x_2 _y_2) (Math|Vector|BreakVector _returnvalue_2))
  ;[1 1 1] Allows the user to rotate the camera when possessing the ball
  (Class|PrimitiveComponent|AddTorqueinDegrees _staticmeshcomponent_2 (Math|Vector|MakeVector 0.0 0.0 (* 1.8e+03 Axis)) "None" true)
  (Transformation|AddLocalRotation _movement_refernce (Math|Rotator|MakeRotator 0.0 0.0 (* Axis (/ (Variables|Default|GetDirection_Force) 5e+01))) false false)
  (Transformation|SetRelativeRotation _springarm (Class|SpringArmComponent|GetTargetRotation _movement_refernce) false false)
  (Transformation|AddLocalRotation _springarm "-30.000000, 0, 0" false false)
  (Physics|SetPhysicsLinearVelocity _staticmeshcomponent_2 (* (Math|Vector|Normalize (+ (Math|Vector|MakeVector _x _y _z) (* (Math|Vector|MakeVector _x_2 _y_2 0.0) (Variables|Default|GetDirection_Force)))) (Math|Vector|VectorLength _returnvalue)) false "None"))

(fn LaunchingBall
  (params (Power :type Float%20%28single-precision%29) (Forward :type Vector) (Direction_Force :type Float%20%28single-precision%29) (Launcher :type BP%20Ball%20Launcher%20Object%20Reference))
  ;[1 1 1] Launches the ball based on power and where the launchers is looking
  (bind _output_get (Variables|Default|SetDirection_Force Direction_Force))
  (Variables|Default|SetLauncher_ref Launcher)
  (Physics|AddForce (Variables|/Script/SummerDeliverables.PossessablePawn|GetStaticMeshComponent (Variables|Default|GetBall_ref)) (* Forward (* Power 1.5e+05)) "None" false))

(fn Bounce
  ;[1 1 1] Allows the ball to bounce a certain amount of times before being destroyed
  (Development|PrintString "Bounce")
  (Variables|Default|SetBounces (+ (Variables|Default|GetBounces) 1))
  (if (> (Variables|Default|GetBounces) (Variables|Default|GetBounce_Max))
    (Class|PossesableComponent|Eject)))