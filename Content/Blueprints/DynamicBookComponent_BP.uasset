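; Movement and scare component for a possessable book, which moves by physics hops.
; Right-axis input turns the mesh and camera, while the top button zeroes velocity and applies an impulse arced by forward input, unless already rising fast.
; The right button scares, swapping to the bad material and blocking jumps until a Tick countdown restores both.
; Each ground-hit call drains stamina, ending possession when it runs out.
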(event EventMoveForwardAxis
  (params (Axis :type Float%20%28single-precision%29))
  (Variables|Default|SetArcForwardPointing Axis))

(event EventMoveRightAxis
  (params (Axis :type Float%20%28single-precision%29))
  (bind _mesh (Variables|Components|GetMesh))
  (bind _camera (Variables|Default|GetCamera))
  (Transformation|AddLocalRotation _mesh (Math|Rotator|MakeRotator 0.0 0.0 (* 2 Axis)) false false)
  (Transformation|SetRelativeRotation _camera (Transformation|GetWorldRotation _mesh) false false)
  (Transformation|AddLocalRotation _camera "-30.000000, 0, 0" false false))

(event EventButtonTop
  (bind _mesh (Variables|Components|GetMesh))
  (bind _mesh_2 (Variables|Components|GetMesh))
  (if (Variables|Default|GetcanJump)
    (bind _returnvalue (Physics|GetPhysicsLinearVelocity _mesh_2 "None"))
    (if (not (> (.z _returnvalue) 1e+02))
      (Physics|SetPhysicsLinearVelocity _mesh_2 (Math|Vector|MakeVector 0.0 0.0 0.0) false "None")
      (Physics|AddImpulse _mesh_2 (+ (* (Math|Vector|GetUpVector _mesh) (Variables|Default|GetJumpScalar)) (* (Math|Vector|GetForwardVector _mesh) (* (Variables|Default|GetArcForwardPointing) (Math|Conversions|ToFloat(Integer) (Variables|Default|GetMovementSpeedScalar))))) "None" false))))

(event EventTick
  (params (DeltaSeconds :type Float%20%28single-precision%29))
  (if (not (Variables|Default|GetcanJump))
    (bind _output_get (Variables|Default|SetcurScareTime (- (Variables|Default|GetcurScareTime) DeltaSeconds)))
    (if (<= _output_get 0.0)
      (Variables|Default|SetcanJump true)
      (bind _aspossessable_book_bp (Utilities|Casting|CastToPossessableBook_BP (Components|GetOwner)))
      (Default|ChangeMat _aspossessable_book_bp (Variables|Default|GetgoodMat)))))

(event EventButtonRight
  (CallFunction|SCARE))

(event EventBeginPlay
  (bind _aspossessable_book_bp (Utilities|Casting|CastToPossessableBook_BP (Components|GetOwner)))
  (Default|ChangeMat _aspossessable_book_bp (Variables|Default|GetgoodMat)))

(fn OnHitGround
  (bind _output_get (Variables|Default|SetStamina%20%28TEMP%29 (- (Variables|Default|GetStamina%20%28TEMP%29) 1)))
  (if (<= _output_get 0)
    (bind _aspossessable_pawn (Utilities|Casting|CastToPossessablePawn (Components|GetOwner)))
    (Class|PossessablePawn|EndPossession _aspossessable_pawn)))

(fn ResetStamina
  (Variables|Default|SetStamina%20%28TEMP%29 3))

(fn SCARE
  (bind _aspossessable_book_bp (Utilities|Casting|CastToPossessableBook_BP (Components|GetOwner)))
  (Default|ChangeMat _aspossessable_book_bp (Variables|Default|GetbadMat))
  (Variables|Default|SetcanJump false)
  (Variables|Default|SetcurScareTime (Variables|Default|GetScareTime)))