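; A possessable bowling ball that a launcher fires and the player then controls.
; On BeginPlay it hands its mesh, movement reference and spring arm to a DynamicBowlingTest_BP possessable component.
; LaunchingBall has the player controller possess the ball, then applies force scaled by power along the given direction.
; Mesh end-overlaps count as bounces; at the limit it tells the Ball_Launcher to reload for the player and destroys itself.
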(event OnComponentEndOverlap(StaticMeshComponent)
  (params (OverlappedComponent :type Primitive%20Component%20Object%20Reference) (OtherActor :type Actor%20Object%20Reference) (OtherComp :type Primitive%20Component%20Object%20Reference) (OtherBodyIndex :type Integer))
  (if (>= (Variables|Default|GetBounces) (Variables|Default|GetBounce_Max))
    (bind _asball_launcher (Utilities|Casting|CastToBall_Launcher (Variables|Default|GetLauncher_ref)))
    (Default|Reloading _asball_launcher (Variables|Default|GetPlayer_ref))
    (Actor|DestroyActor)
    (else
      (Variables|Default|SetBounces (+ (Variables|Default|GetBounces) 1)))))

(event EventBeginPlay
  (|CallParentFunction)
  (bind _asdynamic_bowling_test_bp (Utilities|Casting|CastToDynamicBowlingTest_BP (Variables|Default|GetPossessableComponent)))
  (Variables|/Game/Blueprints/DynamicBowlingTest_BP.DynamicBowlingTest_BP_C|SetMesh _asdynamic_bowling_test_bp (Variables|Default|GetStaticMeshComponent))
  (Variables|/Game/Blueprints/DynamicBowlingTest_BP.DynamicBowlingTest_BP_C|SetForward _asdynamic_bowling_test_bp (Variables|Default|GetMovement%20Refrence))
  (Variables|/Game/Blueprints/DynamicBowlingTest_BP.DynamicBowlingTest_BP_C|SetCamera _asdynamic_bowling_test_bp (Variables|Default|GetSpringArm)))

(event Collision|EventActorBeginOverlap
  (params (OtherActor :type Actor%20Object%20Reference))
  (|CallParentFunction OtherActor))

(event EventTick
  (params (DeltaSeconds :type Float%20%28single-precision%29))
  (|CallParentFunction DeltaSeconds))

(fn ConstructionScript
  (|CallParentFunction))

(fn LaunchingBall
  (params (Power :type Float%20%28single-precision%29) (Forward :type Vector) (Player_ref :type Controller%20Object%20Reference) (Launcher_ref :type Actor%20Object%20Reference))
  (Variables|Default|SetLauncher_ref Launcher_ref)
  (bind _output_get (Variables|Default|SetPlayer_ref Player_ref))
  (bind _asplayer_controller (Utilities|Casting|CastToPlayerController _output_get))
  (Pawn|Possess _asplayer_controller self)
  (Physics|AddForce (Variables|Default|GetStaticMeshComponent) (* Forward (* Power 5e+04)) "None" false))