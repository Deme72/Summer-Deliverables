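; Paranoia base Blueprint that makes its owner jitter in rotation while IsInUse returns true.
; BeginPlay caches the owner's starting roll, pitch and yaw as a fixed baseline.
; Tick passes through a short Delay, throttling updates, then sets the owner's rotation to that baseline plus a small random offset on each axis, so the shake does not accumulate.
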(event EventBeginPlay
  (bind _returnvalue (Components|GetOwner))
  (bind _returnvalue_2 (Transformation|GetActorRotation _returnvalue))
  (bind (_roll _pitch _yaw) (Math|Rotator|BreakRotator _returnvalue_2))
  (Variables|Default|Setx _roll)
  (Variables|Default|Sety _pitch)
  (Variables|Default|Setz _yaw))

(event EventTick
  (params (DeltaSeconds :type Float%20%28single-precision%29))
  (if (Class|InteractableComponent|IsinUse)
    (Utilities|FlowControl|Delay 0.1)
    (Transformation|SetActorRotation (Components|GetOwner) (Math|Rotator|MakeRotator (+ (Variables|Default|Getx) (Math|Random|RandomFloatinRange -5.0 5.0)) (+ (Variables|Default|Gety) (Math|Random|RandomFloatinRange -5.0 5.0)) (+ (Variables|Default|Getz) (Math|Random|RandomFloatinRange -5.0 5.0))))))