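; Component for the possessable crank tank prop, toggled between driving and projectile-scare modes.
; Driving compares successive stick-vector angles as two crank levers, combining their directions into forward movement or yaw.
; In stationary mode, holding Scare builds charge and releasing lobs a projectile at charge-scaled velocity; ActivateScare scares at its location.
; When not charging or past the charge cap, stationary mode ejects and flags blown-out, adjusting stamina each tick.
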(event EventBeginPlay
  (Variables|Default|SetisMoving true))

(event EventTick
  (params (DeltaSeconds :type Float%20%28single-precision%29))
  (|isBlownOutCheck)
  (Utilities|IsMovingState
    (:True
      (|LeftLeverSetting)
      (|RightLeverSetting)
      (|CalculateDirectionsBothLinearAndRotational)
      (|MovingProp))
    (:False
      (|Charge DeltaSeconds))))

(event EventLookRightAxis
  (params (Axis :type Float%20%28single-precision%29))
  (Utilities|IsMovingState
    (:True
      (Variables|Default|SetnewRightVec (Class|KismetMathLibrary|NormalSafe2D (Math|Vector2D|MakeVector2D Axis (stale EventLookUpAxis Axis)) 0.0)))))

(event EventLookUpAxis
  (params (Axis :type Float%20%28single-precision%29))
  (Utilities|IsMovingState
    (:True
      (Variables|Default|SetnewRightVec (Class|KismetMathLibrary|NormalSafe2D (Math|Vector2D|MakeVector2D (stale EventLookRightAxis Axis) Axis) 0.0)))))

(event EventMoveForwardAxis
  (params (Axis :type Float%20%28single-precision%29))
  (Utilities|IsMovingState
    (:True
      (Variables|Default|SetnewLeftVec (Class|KismetMathLibrary|NormalSafe2D (Math|Vector2D|MakeVector2D (stale EventMoveRightAxis Axis) Axis) 0.0)))))

(event EventMoveRightAxis
  (params (Axis :type Float%20%28single-precision%29))
  (Utilities|IsMovingState
    (:True
      (Variables|Default|SetnewLeftVec (Class|KismetMathLibrary|NormalSafe2D (Math|Vector2D|MakeVector2D Axis (stale EventMoveForwardAxis Axis)) 0.0)))))

(event EventMoveButton
  (Variables|Default|SetisMoving (not (Variables|Default|GetisMoving))))

(event EventScareButton
  (Utilities|IsMovingState
    (:False
      (Variables|Default|SetisCharging true)
      (Variables|Default|SetchargeLevel 0.0))))

(event EventScareButtonRelease
  (Utilities|IsMovingState
    (:False
      (Variables|Default|SetisCharging false)
      (CallFunction|Fire))))

(fn GetStaticMesh
  (bind _aspossessable_pawn (Utilities|Casting|CastToPossessablePawn (Components|GetOwner)))
  (return (Variables|/Script/SummerDeliverables.PossessablePawn|GetStaticMeshComponent _aspossessable_pawn)))

(fn ActivateScare
  (params (Projectile :type BP%20Projectile%20Object%20Reference))
  (bind _asbp_crank_tank (Utilities|Casting|CastToBP_CrankTank (Components|GetOwner)))
  (Transformation|SetWorldLocation (Variables|/Game/Blueprints/BP_CrankTank.BP_CrankTank_C|GetScareBounds _asbp_crank_tank) (Transformation|GetWorldLocation (Variables|/Game/Blueprints/BP_Projectile.BP_Projectile_C|GetSphere Projectile)) false false)
  (Class|PossesableComponent|Scare 1.0))

(fn Fire
  (bind _returnvalue (Components|GetOwner))
  (bind _asbp_crank_tank (Utilities|Casting|CastToBP_CrankTank _returnvalue))
  (bind _returnvalue_2 (Game|SpawnActorfromClass "/Game/Blueprints/BP_Projectile.BP_Projectile_C" (Math|Conversions|ToTransform(Vector) (Transformation|GetWorldLocation (Variables|/Game/Blueprints/BP_CrankTank.BP_CrankTank_C|GetlaunchPos _asbp_crank_tank))) "AlwaysSpawn" _returnvalue 0))
  (Default|AssignTank _returnvalue_2 self)
  (bind _staticmesh (CallFunction|GetStaticMesh))
  (if (not (Game|IsActorBeingDestroyed _returnvalue_2))
    (Physics|SetPhysicsLinearVelocity (Variables|/Game/Blueprints/BP_Projectile.BP_Projectile_C|GetSphere _returnvalue_2) (* (Math|Vector|Normalize (+ (Math|Vector|GetForwardVector _staticmesh) (Math|Vector|GetUpVector _staticmesh))) (* (Variables|Default|GetchargeLevel) (Variables|Default|GetlaunchVel))) false "None")))