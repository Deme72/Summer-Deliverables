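; AOE_ability is an actor Blueprint that procedurally builds a vertical column of copies of one mesh, with no area-of-effect logic despite its name.
; The Construction Script adds NumItems static mesh components using Item and stores them in ItemsArray.
; Each copy gets a swept, teleporting Z offset of its index times the mesh bounding box's minimum Z.
; The Event Graph holds only disabled placeholder events.
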(event EventBeginPlay)

(event Collision|EventActorBeginOverlap
  (params (OtherActor :type Actor%20Object%20Reference)))

(event EventTick
  (params (DeltaSeconds :type Float%20%28single-precision%29)))

(fn ConstructionScript
  (for _index (range 1 (Variables|Default|GetNum_items))
    (bind _returnvalue (AddComponent|AddStaticMeshComponent false))
    (Components|StaticMesh|SetStaticMesh _returnvalue (Variables|Default|GetItem))
    (Transformation|AddLocalOffset _returnvalue (Math|Vector|MakeVector 0.0 0.0 (* _index (.z (.Min (Utilities|Struct|BreakBox (StaticMesh|GetBoundingBox (Variables|Default|GetItem))))))) true true)
    (Utilities|Array|Add (Variables|Default|GetItemsArray) _returnvalue)))