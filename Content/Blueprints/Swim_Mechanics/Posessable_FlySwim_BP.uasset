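; Possessable physics pawn that swims by forward impulses while hovering above surfaces, with gravity switched off during possession.
; While possessed, Tick uses a downward sphere trace to adjust height and clamps horizontal velocity.
; Non-plate hits while possessed decrement PlateCount to a minimum of one.
; Left trigger triggers GoBoom, hiding the mesh and launching that many Plate_boy actors from random surrounding points.
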(event OnComponentHit(StaticMesh)
  (params (HitComponent :type Primitive%20Component%20Object%20Reference) (OtherActor :type Actor%20Object%20Reference) (OtherComp :type Primitive%20Component%20Object%20Reference) (NormalImpulse :type Vector :default "0, 0, 0") (Hit :type Hit%20Result%20Structure%20%28by%20ref%29))
  (CallFunction|ReduceDamage OtherActor))

(event EventBeginPlay
  (bind _staticmesh (Variables|Default|GetStaticMesh))
  (|CallParentFunction)
  (Physics|SetEnableGravity _staticmesh true)
  (Variables|Default|Setposs false)
  (Variables|Default|SetStarting_Transform (Transformation|GetWorldTransform _staticmesh)))

(event Collision|EventActorBeginOverlap
  (params (OtherActor :type Actor%20Object%20Reference))
  (|CallParentFunction OtherActor) ; This node is disabled and will not be called.\nDrag off pins to build functionality.
)

(event EventTick
  (params (DeltaSeconds :type Float%20%28single-precision%29))
  (|CallParentFunction DeltaSeconds)
  (CallFunction|MotionControl (Variables|Default|GetMax_Velocity)))

(event EventPossessed
  (params (NewController :type Controller%20Object%20Reference))
  (Variables|Default|Setposs true)
  (Physics|SetEnableGravity (Variables|Default|GetStaticMesh) false))

(event EventUnpossessed
  (params (OldController :type Controller%20Object%20Reference))
  (Variables|Default|Setposs false)
  (Physics|SetEnableGravity (Variables|Default|GetStaticMesh) true))

(event Input|ActionEvents|InputActionFaceButtonBottom
  (params (Key :type Key%20Structure :default "None"))
  (:Pressed
    (CallFunction|Swim (Variables|Default|GetSwim_speed))))

(event Input|ActionEvents|InputActionLeftTrigger
  (params (Key :type Key%20Structure :default "None"))
  (:Pressed
    (CallFunction|GoBoom)))

(event Input|AxisEvents|InputAxisTurn
  (params (AxisValue :type Float%20%28single-precision%29))
  ;[1 1 1] Turn's the current pawn based on camera
  (Pawn|Input|AddControllerYawInput AxisValue))

(fn ConstructionScript
  (Variables|Default|SetPossessableComponent (Variables|Default|GetPosessable_FS_component_BP))
  (|CallParentFunction))

(fn Swim
  (params (Swim_speed :type Float%20%28single-precision%29))
  ;[1 1 1] Forward motion
  (Physics|AddImpulse (Variables|Default|GetStaticMesh) (* (Math|Vector|GetForwardVector (Variables|Default|GetForward)) Swim_speed) "None" true))

(fn MotionControl
  (params (MaxVel :type Float%20%28single-precision%29))
  (bind _staticmesh (Variables|Default|GetStaticMesh))
  (bind _returnvalue (Transformation|GetWorldLocation _staticmesh))
  (if (Variables|Default|Getposs)
    ;[1 1 1] This mess handles height above object
    (bind _outhit (Collision|SphereTraceByChannel _returnvalue (+ _returnvalue (* (* (Math|Vector|GetUpVector _staticmesh) -1.0) 3e+02)) (.x (.Max (Components|StaticMesh|GetLocalBounds (Variables|Default|GetStaticMesh)))) "TraceTypeQuery1" false 0 "ForDuration" true "(R=1.000000,G=0.000000,B=0.000000,A=1.000000)" "(R=0.000000,G=1.000000,B=0.000000,A=1.000000)" 0.0))
    (Utilities|Casting|CastToPlate_boy (.HitActor (Collision|BreakHitResult _outhit))
      (:CastFailed
        (Transformation|AddWorldOffset (Variables|Default|GetStaticMesh) (Math|Vector|MakeVector 0.0 0.0 (- (Variables|Default|GetMax_height) (.Distance (Collision|BreakHitResult _outhit)))) true true)
        (CallFunction|VelocityLimitation MaxVel)))))

(fn VelocityLimitation
  (params (InputPin :type Float%20%28single-precision%29))
  (bind _returnvalue (Transformation|GetVelocity))
  (bind _returnvalue_2 (Math|Vector|MakeVector (.x _returnvalue) (.y _returnvalue) 0.0))
  (bind _returnvalue_3 (Math|Vector|ClampVectorSize _returnvalue_2 0.0 InputPin))
  (if (> (Math|Vector|VectorLength _returnvalue_2) InputPin)
    (Physics|SetPhysicsLinearVelocity (Variables|Default|GetStaticMesh) (Math|Vector|MakeVector (.x _returnvalue_3) (.y _returnvalue_3) (.z _returnvalue)) false "None")))

(fn GoBoom
  (bind _returnvalue (Math|Random|RandomFloatinRange 0.0 359.0))
  (bind _staticmesh (Variables|Default|GetStaticMesh))
  (bind _staticmesh_2 (Variables|Default|GetStaticMesh))
  (bind _returnvalue_2 (Transformation|GetWorldTransform _staticmesh))
  (bind _returnvalue_3 (Math|Trig|Cos(Degrees) _returnvalue))
  (bind _returnvalue_4 (Math|Trig|Sin(Degrees) _returnvalue))
  (bind _max (Components|StaticMesh|GetLocalBounds _staticmesh_2))
  (bind _returnvalue_5 (Transformation|GetWorldLocation _staticmesh))
  (bind _returnvalue_6 (+ (.x _max) 4.0))
  (bind _returnvalue_7 (* _returnvalue_3 _returnvalue_6))
  (bind _returnvalue_8 (* _returnvalue_4 _returnvalue_6))
  (bind _returnvalue_9 (+ (.x _returnvalue_5) _returnvalue_7))
  (bind _returnvalue_10 (+ (.y _returnvalue_5) _returnvalue_8))
  (bind _returnvalue_11 (Math|Vector|MakeVector _returnvalue_9 _returnvalue_10 (.z _returnvalue_5)))
  (Rendering|SetVisibility (Variables|Default|GetStaticMesh) false false)
  (for _index (range 1 (Variables|Default|GetPlate_count))
    (bind _returnvalue_12 (Game|SpawnActorfromClass "/Game/Blueprints/Swim_Mechanics/Plate_boy.Plate_boy_C" (Math|Transform|MakeTransform _returnvalue_11 (.rotation _returnvalue_2) (.scale _returnvalue_2)) "Undefined" self 0))
    (Physics|AddImpulse (Variables|/Game/Blueprints/Swim_Mechanics/Plate_boy.Plate_boy_C|GetShape_Torus _returnvalue_12) (* (- (Transformation|GetWorldLocation _staticmesh) _returnvalue_11) (Variables|Default|GetPlate_Speed)) "None" true))
  (Development|PrintString "Do Eject"))

(fn ReduceDamage
  (params (Object :type Object%20Object%20Reference))
  (if (Variables|Default|Getposs)
    (Utilities|Casting|CastToPlate_boy Object
      (:CastFailed
        (bind _output_get (Variables|Default|SetPlate_count (- (Variables|Default|GetPlate_count) 1)))
        (if (<= _output_get 1)
          (Variables|Default|SetPlate_count 1))
        (Development|PrintString (Utilities|String|Append "Damage: " (Utilities|String|ToString(Integer) _output_get)))))))