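; Possessable-prop component for BP_SimonSays that runs a Simon Says input minigame to power the prop's scare.
; Interacting generates a short random code, matched against button, trigger and movement inputs with a cooldown between checked presses.
; Completing it enables scaring and raises the multiplier more for faster entry, capped on Tick; mistakes lower it and reroll.
; While possessed, codes also reroll on timeout; progress shows only through debug prints.
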(event EventBeginPlay)

(event EventTick
  (params (DeltaSeconds :type Float%20%28single-precision%29))
  (if (Variables|Default|GetInProp)
    (Variables|Default|SetmInputCooldown (- (Variables|Default|GetmInputCooldown) DeltaSeconds))
    (if (> (Variables|Default|GetmScare_Mult) 2.0)
      (Variables|Default|SetmScare_Mult 2.0))
    (bind _output_get (Variables|Default|SetmTime_For_Sequence (+ (Variables|Default|GetmTime_For_Sequence) (Utilities|Time|GetWorldDeltaSeconds))))
    (Development|PrintString (Utilities|String|ToString(Float) _output_get) true false)
    (if (> (Variables|Default|GetmTime_For_Sequence) 15.0)
      (CallFunction|GenerateSequence)
      (Variables|Default|SetmTime_For_Sequence 0.0))))

(event EventMoveForwardAxis
  (params (Axis :type Float%20%28single-precision%29))
  ;[1 1 1] Handles the input for the code sequence
  (if (!= Axis 0.0)
    (if (< Axis 0.0)
      (CallFunction|CheckSequence "Back_Move")
      (else
        (CallFunction|CheckSequence "Forward_Move")))))

(event EventEndInteract
  (Variables|Default|SetInProp false))

(event EventScareButton
  (if (Variables|Default|GetmCan_Scare)
    (Class|PossesableComponent|Scare (Variables|Default|GetmScare_Mult))))

(event EventOnInteract
  (bind _aspossessable_pawn (Utilities|Casting|CastToPossessablePawn (Components|GetOwner)))
  (bind _asbp_simon_says (Utilities|Casting|CastToBP_SimonSays _aspossessable_pawn))
  (Variables|Default|SetmCodeReadRef _asbp_simon_says)
  (CallFunction|GenerateSequence)
  (Variables|Default|SetInProp true))

(event EventLookRightAxis
  (params (Axis :type Float%20%28single-precision%29))
  (Transformation|AddWorldRotation (Variables|/Game/Blueprints/BP_SimonSays.BP_SimonSays_C|GetSpringArm (Variables|Default|GetmCodeReadRef)) (Math|Rotator|MakeRotator 0.0 0.0 (* Axis (* (Utilities|Time|GetWorldDeltaSeconds) 5e+01))) false false))

(event EventButtonTop
  ;[1 1 1] Handles the input for the code sequence
  (CallFunction|CheckSequence "Button_Top"))

(event EventMoveButton
  ;[1 1 1] Handles the input for the code sequence
  (CallFunction|CheckSequence "Button_Down"))

(event EventLeftTrigger
  ;[1 1 1] Handles the input for the code sequence
  (CallFunction|CheckSequence "Left_Trigger"))

(event EventRightTrigger
  ;[1 1 1] Handles the input for the code sequence
  (CallFunction|CheckSequence "Right_Trigger"))

(event EventMoveRightAxis
  (params (Axis :type Float%20%28single-precision%29))
  ;[1 1 1] Handles the input for the code sequence
  (if (!= Axis 0.0)
    (if (< Axis 0.0)
      (CallFunction|CheckSequence "Left_Move")
      (else
        (CallFunction|CheckSequence "Right_Move")))))

(fn GenerateSequence
  (Utilities|Array|Clear (Variables|Default|GetmCode_String))
  (Variables|Default|SetmIndex 0)
  (for _index (range 0 (Math|Random|RandomIntegerinRange 1 2))
    (bind _output_get (Variables|Default|Settemp (Utilities|Array|Get(acopy) (Variables|Default|GetmString_Gen) (Math|Random|RandomIntegerinRange 0 (Variables|Default|GetmNum_inputs)))))
    (Utilities|Array|Add (Variables|Default|GetmCode_String) _output_get)
    (Development|PrintString _output_get false)))

(fn CheckSequence
  (params (Input :type String))
  (bind _mindex (Variables|Default|GetmIndex))
  (bind _mindex_2 (Variables|Default|GetmIndex))
  (bind _mcode_string (Variables|Default|GetmCode_String))
  (bind _returnvalue (Utilities|Array|Length _mcode_string))
  (bind _returnvalue_2 (+ _mindex_2 1))
  (bind _returnvalue_3 (< _mindex _returnvalue))
  (if (<= (Variables|Default|GetmInputCooldown) 0.0)
    (if _returnvalue_3
      (if (Utilities|Enum|Equal(Enum) (Utilities|Array|Get(acopy) (Variables|Default|GetmCode_String) _mindex) Input)
        (if _returnvalue_3
          (Development|PrintString "success")
          (if (< _returnvalue_2 (Utilities|Array|Length (Variables|Default|GetmCode_String)))
            (Development|PrintString (Utilities|Array|Get(acopy) (Variables|Default|GetmCode_String) _returnvalue_2) true false))
          (Math|Integer|IncrementInt _mindex
            (:%20%20
              (if (< (Variables|Default|GetmIndex) (Utilities|Array|Length (Variables|Default|GetmCode_String)))
                _
                (else
                  (bind _output_get (Variables|Default|SetmScare_Mult (+ (Variables|Default|GetmScare_Mult) (* (/ 7.0 (Variables|Default|GetmTime_For_Sequence)) 0.5))))
                  (Variables|Default|SetmCan_Scare true)
                  (CallFunction|GenerateSequence)
                  (Development|PrintString (Utilities|String|ToString(Float) _output_get) false)
                  (Variables|Default|SetmTime_For_Sequence 0.0)))
              (CallFunction|AddCooldown :!label _label))))
        (else
          (CallFunction|GenerateSequence)
          (Variables|Default|SetmScare_Mult (- (Variables|Default|GetmScare_Mult) 0.5))
          (goto _label))))))

(fn AddCooldown
  (Variables|Default|SetmInputCooldown 1.5))