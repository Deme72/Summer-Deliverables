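; Possessable pawn that the player steers as either a mobile body or a stationary projectile shooter, with gravity off on its mesh.
; The bottom face button toggles movement and shooting modes after a delay, leveling the view for movement.
; Left trigger spawns a forward-pushed projectile, and firing during cooldown prints "Jammed!" and restarts the timer.
; Yaw always works, pitch is blocked while moving, and possession events are empty.
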(event EventBeginPlay
  (bind _staticmesh (Variables|Default|GetStaticMesh))
  (|CallParentFunction)
  (Physics|SetEnableGravity _staticmesh false)
  (Variables|Default|Setposs false)
  (Variables|Default|SetStarting_Transform (Transformation|GetWorldTransform _staticmesh)))

(event Collision|EventActorBeginOverlap
  (params (OtherActor :type Actor%20Object%20Reference))
  (|CallParentFunction OtherActor) ; This node is disabled and will not be called.\nDrag off pins to build functionality.
)

(event EventTick
  (params (DeltaSeconds :type Float%20%28single-precision%29))
  (|CallParentFunction DeltaSeconds)
  (Variables|Default|SetShotTimer (Math|Float|Max(Float) (- (Variables|Default|GetShotTimer) DeltaSeconds) 0.0)))

(event EventPossessed
  (params (NewController :type Controller%20Object%20Reference)))

(event EventUnpossessed
  (params (OldController :type Controller%20Object%20Reference)))

(event Input|ActionEvents|InputActionFaceButtonBottom
  (params (Key :type Key%20Structure :default "None"))
  (bind _returnvalue (Pawn|GetController))
  ;[1 1 1] Switch Modes
  (:Pressed
    (if (not (Variables|Default|GetInStateTransition))
      (Variables|Default|SetInStateTransition true)
      (if (Variables|Default|GetCanShoot)
        (Development|PrintString "Preparing to Move")
        (Variables|Default|SetCanShoot false)
        (Utilities|FlowControl|Delay (Variables|Default|GetModeSwitchTime))
        (Variables|Default|SetCanMove true)
        (Pawn|SetControlRotation _returnvalue (Math|Rotator|MakeRotator 0.0 0.0 (.Yaw (Math|Rotator|BreakRotator (Pawn|GetControlRotation _returnvalue :!class /Script/Engine.Controller)))))
        (Development|PrintString "Ready to Move")
        (else
          (Development|PrintString "Preparing to Shoot")
          (Variables|Default|SetCanMove false)
          (Utilities|FlowControl|Delay (Variables|Default|GetModeSwitchTime))
          (Variables|Default|SetCanShoot true)
          (Development|PrintString "Ready to Shoot")))
      (Variables|Default|SetInStateTransition false))))

(event Input|ActionEvents|InputActionLeftTrigger
  (params (Key :type Key%20Structure :default "None"))
  ;[1 1 1] Shoot (In Shooting Mode)
  (:Pressed
    (if (Variables|Default|GetCanShoot)
      (if (<= (Variables|Default|GetShotTimer) 0.0)
        (Development|PrintString "Shooting!")
        (CallFunction|ShootProjectile)
        (else
          (Development|PrintString "Jammed!")))
      (Variables|Default|SetShotTimer (Variables|Default|GetShotCooldown)))))

(event Input|AxisEvents|InputAxisTurn
  (params (AxisValue :type Float%20%28single-precision%29))
  ;[1 1 1] Turn's the current pawn based on camera
  (Pawn|Input|AddControllerYawInput AxisValue))

(event Input|AxisEvents|InputAxisMoveForward
  (params (AxisValue :type Float%20%28single-precision%29))
  ;[1 1 1] Move (In Movement Mode)
  (if (Variables|Default|GetCanMove)
    (Transformation|AddActorLocalOffset (* (Math|Vector|MakeVector AxisValue 0.0 0.0) (Variables|Default|GetMove_speed)) true true)))

(event Input|AxisEvents|InputAxisMoveRight
  (params (AxisValue :type Float%20%28single-precision%29))
  ;[1 1 1] Move (In Movement Mode)
  (if (Variables|Default|GetCanMove)
    (Transformation|AddActorLocalOffset (* (Math|Vector|MakeVector 0.0 AxisValue 0.0) (Variables|Default|GetMove_speed)) true false)))

(event Input|AxisEvents|InputAxisLookUp
  (params (AxisValue :type Float%20%28single-precision%29))
  (if (not (Variables|Default|GetCanMove))
    (Pawn|Input|AddControllerPitchInput AxisValue)))

(fn ConstructionScript
  (Variables|Default|SetPossessableComponent (Variables|Default|GetPosessable_FS_component_BP))
  (|CallParentFunction))

(fn ShootProjectile
  (bind _returnvalue (Transformation|GetActorRotation))
  (bind _returnvalue_2 (Math|Vector|GetForwardVector _returnvalue))
  (bind _returnvalue_3 (Game|SpawnActorfromClass "/Game/Blueprints/Shoot_Mechanics/Projectile.Projectile_C" (Math|Transform|MakeTransform (+ (Transformation|GetActorLocation) (* _returnvalue_2 (.x (.Max (Components|StaticMesh|GetLocalBounds (Variables|Default|GetStaticMesh)))))) "0, 0, 0" "0.500000,0.500000,0.500000") "Undefined" 0 0))
  (Physics|AddForce (Variables|/Game/Blueprints/Shoot_Mechanics/Projectile.Projectile_C|GetShape_Torus _returnvalue_3) (* _returnvalue_2 (Variables|Default|GetProjectile_speed)) "None" true))