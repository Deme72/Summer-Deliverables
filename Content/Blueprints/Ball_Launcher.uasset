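; Ball launcher actor that the player aims by turning left and right, with a golf bar mini-game UI attached.
; On BeginPlay it creates the GolfBarMiniGame widget, stores a reference, adds it to the viewport and hides it.
; The MoveRight input axis feeds TurningLauncher, which applies the raw axis value as a local yaw rotation, without delta-time scaling.
; No launch logic or code to reveal the widget is present in these graphs.
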(event EventBeginPlay
  (|CallParentFunction)
  (bind _returnvalue (UserInterface|CreateWidget "/Game/UI_Widgets/GolfBarMiniGame.GolfBarMiniGame_C"))
  (bind _output_get (Variables|Default|SetGolf%20Bar%20UI%20Ref _returnvalue))
  (UserInterface|Viewport|AddtoViewport _output_get 0)
  (Widget|SetVisibility _output_get "Hidden"))

(event Collision|EventActorBeginOverlap
  (params (OtherActor :type Actor%20Object%20Reference))
  (|CallParentFunction OtherActor) ; This node is disabled and will not be called.\nDrag off pins to build functionality.
)

(event EventTick
  (params (DeltaSeconds :type Float%20%28single-precision%29))
  (|CallParentFunction DeltaSeconds) ; This node is disabled and will not be called.\nDrag off pins to build functionality.
)

(event Input|AxisEvents|InputAxisMoveRight
  (params (AxisValue :type Float%20%28single-precision%29))
  (CallFunction|TurningLauncher AxisValue))

(fn ConstructionScript
  (|CallParentFunction))

(fn TurningLauncher
  (params (Rotate_amount :type Float%20%28single-precision%29))
  (Transformation|AddActorLocalRotation (Math|Rotator|MakeRotator 0.0 0.0 Rotate_amount) false false))