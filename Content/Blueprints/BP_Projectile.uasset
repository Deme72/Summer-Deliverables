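; BP_Projectile is a projectile actor that triggers a scare on its assigned tank when it overlaps something.
; AssignTank stores the Tank reference and prints its name to the screen.
; On overlap with any actor other than a BP_CrankTank, it calls ActivateScare on that stored Tank, passing itself, then destroys itself.
; Overlaps with any BP_CrankTank are ignored, and no movement logic appears in the graphs.
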(event EventBeginPlay)

(event EventTick
  (params (DeltaSeconds :type Float%20%28single-precision%29)))

(event Collision|EventActorBeginOverlap
  (params (OtherActor :type Actor%20Object%20Reference))
  (Utilities|Casting|CastToBP_CrankTank OtherActor
    (:CastFailed
      (Default|ActivateScare (Variables|Default|GetTank) self)
      (Actor|DestroyActor))))

(fn ConstructionScript)

(fn AssignTank
  (params (myTank :type Crank%20Tank%20Component%20Object%20Reference))
  (bind _output_get (Variables|Default|SetTank myTank))
  (Development|PrintString (Utilities|GetDisplayName _output_get)))