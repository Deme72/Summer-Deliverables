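; Actor component that flickers its owner's spot light when an EndInteract event fires.
; BeginPlay caches the owner's SpotLightComponent.
; EndInteract picks a random even toggle count, then loops through short random delays, using a FlipFlop to alternate the light's visibility.
; When the countdown ends, the light is forced visible.
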(event EventBeginPlay
  (Variables|Default|SetLight (Actor|GetComponentbyClass (Components|GetOwner) "/Script/Engine.SpotLightComponent")))

(event EventEndInteract
  (bind _light (Variables|Default|GetLight))
  (Variables|Default|SetIndex (* (Math|Random|RandomIntegerinRange 4 8) 2))
  (if (> (Variables|Default|GetIndex) 0) :!label _label
    (Utilities|FlowControl|Delay (Math|Random|RandomFloatinRange 0.05 0.3))
    (bind _isa (Utilities|FlowControl|FlipFlop)
      (:A
        _)
      (:B
        _))
    (Rendering|SetVisibility _light _isa false)
    (Math|Integer|DecrementInt (Variables|Default|GetIndex)
      (:%20%20
        (goto _label)))
    (else
      (Rendering|SetVisibility _light true false))))