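; BP_CL_MillWorkBuilder is a construction-script builder for a modular 5x5 room unit with optional walls, ceiling, floor and light.
; Walls A–D each pick a structure mesh and can add an extension mesh chosen by the shared WallHeight, which also sets ceiling elevation.
; Disabled parts have their components destroyed, while an enabled light is set invisible.
; The WindowSingle option resolves to the plain wall mesh, and the AllExtension logic is unconnected.
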(event EventBeginPlay)

(event Collision|EventActorBeginOverlap
  (params (OtherActor :type Actor%20Object%20Reference)))

(event EventTick
  (params (DeltaSeconds :type Float%20%28single-precision%29)))

(fn ConstructionScript
  (bind _sm_ceiling_5x5 (Variables|Default|GetSM_Ceiling_5x5))
  (bind _unit_light_sp (Variables|Default|GetUnit_Light_SP))
  (bind _wallheight (Variables|WallSection|GetWallHeight))
  (bind _vwallext_a (Variables|Default|GetvWallExt_A))
  (bind _sm_floor_5x5 (Variables|Default|GetSM_Floor_5x5))
  (bind _vwallstructure_a (Variables|Default|GetvWallStructure_A))
  (bind _returnvalue (Utilities|Select :Index _wallheight :NewEnumerator0 0 :NewEnumerator1 1 :NewEnumerator2 2 :NewEnumerator3 3))
  (bind _output (Utilities|Array|Get(acopy) _vwallext_a _returnvalue))
  (Utilities|FlowControl|Sequence
    (:then_0
      ;[1 1 1] Which Wall
      (if (Variables|WallSection|GetA)
        ;[1 1 1] Which Wall Type
        (Components|StaticMesh|SetStaticMesh (Variables|Default|GetSM_Wall_5x3_A) (Utilities|Array|Get(acopy) _vwallstructure_a (Utilities|Select :Index (Variables|WallSection|GetWallStructure_A) :NewEnumerator0 0 :NewEnumerator1 1 :NewEnumerator2 2 :NewEnumerator3 0)))
        (if (Variables|WallSection|GetA%20Extension)
          ;[1 1 1] Wall Ext
          (Components|StaticMesh|SetStaticMesh (Variables|Default|GetSM_Wall_Ext_5x1_A) _output)
          (else
            ;[1 1 1] Deletes Unwanted Components
            (Components|DestroyComponent (Variables|Default|GetSM_Wall_Ext_5x1_A) :!label _label)))
        (else
          (Components|DestroyComponent (Variables|Default|GetSM_Wall_5x3_A))
          (goto _label))))
    (:then_1
      (if (Variables|WallSection|GetB)
        (Components|StaticMesh|SetStaticMesh (Variables|Default|GetSM_Wall_5x3_B) (Utilities|Array|Get(acopy) _vwallstructure_a (Utilities|Select :Index (Variables|WallSection|GetWallStructure_B) :NewEnumerator0 0 :NewEnumerator1 1 :NewEnumerator2 2 :NewEnumerator3 0)))
        (if (Variables|WallSection|GetB%20Extension)
          (Components|StaticMesh|SetStaticMesh (Variables|Default|GetSM_Wall_Ext_5x1_B) _output)
          (else
            (Components|DestroyComponent (Variables|Default|GetSM_Wall_Ext_5x1_B) :!label _label_2)))
        (else
          (Components|DestroyComponent (Variables|Default|GetSM_Wall_5x3_B))
          (goto _label_2))))
    (:then_2
      (if (Variables|WallSection|GetC)
        (Components|StaticMesh|SetStaticMesh (Variables|Default|GetSM_Wall_5x3_C) (Utilities|Array|Get(acopy) _vwallstructure_a (Utilities|Select :Index (Variables|WallSection|GetWallStructure_C) :NewEnumerator0 0 :NewEnumerator1 1 :NewEnumerator2 2 :NewEnumerator3 0)))
        (if (Variables|WallSection|GetC%20Extension)
          (Components|StaticMesh|SetStaticMesh (Variables|Default|GetSM_Wall_Ext_5x1_C) _output)
          (else
            (Components|DestroyComponent (Variables|Default|GetSM_Wall_Ext_5x1_C) :!label _label_3)))
        (else
          (Components|DestroyComponent (Variables|Default|GetSM_Wall_5x3_C))
          (goto _label_3))))
    (:then_3
      (if (Variables|WallSection|GetD)
        (Components|StaticMesh|SetStaticMesh (Variables|Default|GetSM_Wall_5x3_D) (Utilities|Array|Get(acopy) _vwallstructure_a (Utilities|Select :Index (Variables|WallSection|GetWallStructure_D) :NewEnumerator0 0 :NewEnumerator1 1 :NewEnumerator2 2 :NewEnumerator3 0)))
        (if (Variables|WallSection|GetD%20Extension)
          (Components|StaticMesh|SetStaticMesh (Variables|Default|GetSM_Wall_Ext_5x1_D) _output)
          (else
            (Components|DestroyComponent (Variables|Default|GetSM_Wall_Ext_5x1_D) :!label _label_4)))
        (else
          (Components|DestroyComponent (Variables|Default|GetSM_Wall_5x3_D))
          (goto _label_4))))
    (:then_4
      ;[1 1 1] Ceiling
      (if (Variables|FloorCeiling|GetCeiling)
        (Components|StaticMesh|SetStaticMesh _sm_ceiling_5x5 (Variables|Default|GetvCeiling))
        (Transformation|SetRelativeLocation _sm_ceiling_5x5 (Math|Vector|MakeVector 0.0 0.0 (* (+ (Math|Conversions|ToFloat(Integer) (Utilities|Select :Index (Variables|WallSection|GetWallHeight) :NewEnumerator0 0 :NewEnumerator1 1 :NewEnumerator2 2 :NewEnumerator3 3)) 3.2) 1e+02)) false false)
        (else
          (Components|DestroyComponent (Variables|Default|GetSM_Ceiling_5x5)))))
    (:then_5
      (if (Variables|FloorCeiling|GetFloor)
        (Components|StaticMesh|SetStaticMesh _sm_floor_5x5 (Variables|Default|GetNewFloorMesh))
        (else
          (Components|DestroyComponent _sm_floor_5x5))))
    (:then_6
      ;[1 1 1] Light
      (if (Variables|FloorCeiling|GetLightVar)
        (Rendering|SetVisibility _unit_light_sp false false)
        (else
          (Components|DestroyComponent _unit_light_sp))))))