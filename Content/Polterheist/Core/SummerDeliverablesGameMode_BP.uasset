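; Game mode for Polterheist that creates local players up to a maximum count and manages their pawn swaps.
; BeginPlay caches PlayerStarts and creates the players with controllers.
; SpawnCharacter replaces a controller's pawn with one built by BP_ActualController, while DespawnCharacter swaps in a BP_InitPawn, both using GetRandomSpawn.
; SpawnPlayers, not called here, instead places a BP_Ghosty per player at the PlayerStart tagged with its index.
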(event Custom|Spawn%20Character
  (params (Player%20Controller :type Player%20Controller%20Object%20Reference))
  (bind _returnvalue (Pawn|GetControlledPawn Player%20Controller))
  ;[1 1 1] Spawn a character at a random player start.
  (Utilities|IsValid _returnvalue
    (:Is%20Valid
      (Actor|DestroyActor _returnvalue)
      (bind _asbp_actual_controller (Utilities|Casting|CastToBP_ActualController Player%20Controller)
        (:then
          (bind _returnvalue_2 (Class|PlayerGhostController|CreatePlayerPawn _asbp_actual_controller (.location (Utilities|GetRandomSpawn))))
          (Pawn|Possess Player%20Controller _returnvalue_2))
        (:CastFailed
          (Development|PrintString "failed to cast Controller to GC_BP"))))))

(event Custom|Despawn%20Character
  (params (Player%20Controller :type Player%20Controller%20Object%20Reference))
  (bind _returnvalue (Pawn|GetControlledPawn Player%20Controller))
  ;[1 1 1] Despawn character.
  (Utilities|IsValid _returnvalue
    (:Is%20Valid
      (Actor|DestroyActor _returnvalue)
      (bind _returnvalue_2 (Game|SpawnActorfromClass "/Game/Polterheist/Core/BP_InitPawn.BP_InitPawn_C" (Utilities|GetRandomSpawn) "AlwaysSpawn" 0 0))
      (Pawn|Possess Player%20Controller _returnvalue_2))))

(event EventBeginPlay
  ;[1 1 1] Gather all PlayerStart points and create empty pawns on them.
  (CallFunction|GetPlayerStartPoints)
  (while (< (Variables|Default|GetPlayerCount) (Variables|Default|GetMaxPlayerCount))
    (Variables|Default|SetPlayerCount (+ (Variables|Default|GetPlayerCount) 1))
    (Class|GameplayStatics|CreatePlayer -1)))

(fn ConstructionScript)

(fn GetPlayerStartPoints
  (bind _outactors (Actor|GetAllActorsOfClass "/Script/Engine.PlayerStart"))
  (bind _output_get (Variables|Default|SetSpawnPoints _outactors))
  (return _output_get))

(fn SpawnPlayers
  (for _index (range 0 (- (Variables|Default|GetMaxPlayerCount) 1))
    (Variables|Default|SetIndex _index)
    (for _array_element (Variables|Default|GetSpawnPoints)
      (if (Utilities|Name|Equal(Name) (Variables|/Script/Engine.PlayerStart|GetPlayerStartTag _array_element) (Utilities|String|StringToName (Utilities|String|ToString(Integer) (Variables|Default|GetIndex))))
        (bind _returnvalue (Class|GameplayStatics|CreatePlayer (Variables|Default|GetIndex)))
        (Utilities|IsValid _returnvalue
          (:Is%20Valid
            (bind _returnvalue_2 (Game|SpawnActorfromClass "/Game/Polterheist/Character/Player/BP_Ghosty.BP_Ghosty_C" (Transformation|GetActorTransform _array_element) "AlwaysSpawn" 0 0))
            (Utilities|IsValid _returnvalue_2
              (:Is%20Valid
                (Pawn|Possess (Game|GetPlayerController (Variables|Default|GetIndex)) _returnvalue_2))
              (:Is%20Not%20Valid
                (Development|PrintString "OOPS" true true "(R=1.000000,G=0.000000,B=0.000000,A=1.000000)" :!label _label))))
          (:Is%20Not%20Valid
            (goto _label)))))))