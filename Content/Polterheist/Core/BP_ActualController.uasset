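; Player controller for Polterheist that toggles the player between spawned and despawned on the StartButton input.
; A FlipFlop alternates between asking SummerDeliverablesGameMode_BP to spawn the character, adding a new stamina-bar HUD to that player's screen, and despawning the character and removing the HUD.
; Unconnected test graphs hold calls for power and accuracy setters and a sample prop control scheme message on the HUD.
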(event Input|ActionEvents|InputActionStartButton
  (params (Key :type Key%20Structure :default "None"))
  (bind _self self)
  ;[1 1 1] Makes start flip between spawn and pause
  (:Pressed
    (Utilities|FlowControl|FlipFlop
      (:A
        ;[1 1 1] Spawn character when Start is pressed
        (bind _assummer_deliverables_game_mode_bp (Utilities|Casting|CastToSummerDeliverablesGameMode_BP (Game|GetGameMode)))
        (Default|SpawnCharacter _assummer_deliverables_game_mode_bp _self)
        ;[1 1 1] Create and add player HUD that holds the stamina bar.
        (bind _returnvalue (UserInterface|CreateWidget "/Game/Polterheist/UI/HUD.HUD_C" _self))
        (bind _output_get (Variables|Default|SetHUD%20Ref _returnvalue))
        (Development|PrintString "Hud Has Been Set")
        (UserInterface|Viewport|AddtoPlayerScreen _output_get))
      (:B
        ;[1 1 1] Despawn character when Options is pressed.
        (bind _assummer_deliverables_game_mode_bp_2 (Utilities|Casting|CastToSummerDeliverablesGameMode_BP (Game|GetGameMode)))
        (Default|DespawnCharacter _assummer_deliverables_game_mode_bp_2 self)
        ;[1 1 1] Remove HUD on Pause screen
        (Utilities|IsValid (Variables|Default|GetHUD%20Ref)
          (:Is%20Valid
            (Widget|RemovefromParent (Variables|Default|GetHUD%20Ref))))))))

(fn ConstructionScript)