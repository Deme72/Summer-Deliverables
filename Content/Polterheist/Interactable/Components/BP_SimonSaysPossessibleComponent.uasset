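; Possessable component for the Simon Says prop in Polterheist, where the possessing player enters random button sequences to charge a scare.
; CheckSequence compares cooldown-gated inputs to the generated code and updates the HUD code reader.
; Faster completions raise the capped scare multiplier and unlock scaring, while mistakes lower it and apply a stamina change.
; Tick regenerates timed-out sequences, and scaring fires the multiplier, ejects the player and resets state.
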(event EventTick
  (params (DeltaSeconds :type Float%20%28single-precision%29))
  (if (Variables|Default|GetInProp)
    (Variables|Default|SetmInputCooldown (- (Variables|Default|GetmInputCooldown) DeltaSeconds))
    (if (> (Variables|Default|GetmScare_Mult) (Variables|Default|GetMaxScare))
      (Variables|Default|SetmScare_Mult (Variables|Default|GetMaxScare)))
    (bind _output_get (Variables|Default|SetmTime_For_Sequence (+ (Variables|Default|GetmTime_For_Sequence) (Utilities|Time|GetWorldDeltaSeconds))))
    (if (> (Variables|Default|GetmTime_For_Sequence) 15.0)
      (CallFunction|GenerateSequence)
      (Variables|Default|SetmTime_For_Sequence 0.0)
      (Class|PossesableComponent|SetStamina (* (Utilities|Time|GetWorldDeltaSeconds) -0.5) true))))

(event EventMoveForwardAxis
  (params (Axis :type Float%20%28single-precision%29))
  ;[1 1 1] Handles the input for the code sequence
  (if (!= Axis 0.0)
    (if (< Axis 0.0)
      (CallFunction|CheckSequence "Back_Move")
      (else
        (CallFunction|CheckSequence "Forward_Move")))))

(event EventEndInteract
  (bind _hud_ref (Variables|Default|GetHUD%20Ref))
  (CallFunction|SetDefaults)
  ;[0 0 1] Remove HUD elements
  (Class|BPIHUDInterface|DestroyCodeReader(Message) _hud_ref)
  (Class|BPIHUDInterface|DestroyPropControlScheme(Message) _hud_ref))

(event EventScareButton
  (bind _hud_ref (Variables|Default|GetHUD%20Ref))
  (if (Variables|Default|GetmCan_Scare)
    (Class|PossesableComponent|Scare (Variables|Default|GetmScare_Mult))
    (Class|PossesableComponent|SetStamina (Variables|Default|GetmFailStam) true)
    (Class|PossesableComponent|Eject)
    ;[0 0 1] Remove HUD elements
    (Class|BPIHUDInterface|DestroyCodeReader(Message) _hud_ref)
    (Class|BPIHUDInterface|DestroyCodeReader(Message) _hud_ref)
    (CallFunction|SetDefaults)))

(event EventOnInteract
  (bind _aspossessable_pawn (Utilities|Casting|CastToPossessablePawn (Components|GetOwner)))
  (bind _asbp_simon_says (Utilities|Casting|CastToBP_SimonSays _aspossessable_pawn))
  (Variables|Default|SetmCodeReadRef _asbp_simon_says)
  (CallFunction|GenerateSequence)
  (Variables|Default|SetInProp true)
  ;[0 0 1] Set up the HUD reference and Create Code Reader UI
  (bind _asbp_actual_controller (Utilities|Casting|CastToBP_ActualController (Class|PossesableComponent|GetCurrentPlayer)))
  (bind _output_get (Variables|Default|SetHUD%20Ref (Variables|/Game/Polterheist/Core/BP_ActualController.BP_ActualController_C|GetHUD%20Ref _asbp_actual_controller)))
  (Class|BPIHUDInterface|MakePropControlScheme(Message) _output_get (Utilities|Array|MakeArray (Utilities|Struct|MakeS_PropControls "/Game/Polterheist/UI/Buttons/T_X.T_X" "Scare") (Utilities|Struct|MakeS_PropControls "/Game/Polterheist/UI/Buttons/T_B.T_B" "Leave Prop")))
  (Class|BPIHUDInterface|MakeCodeReader(Message) _output_get (Variables|Default|GetmCode_String))
  (Class|BPIHUDInterface|UpdateCodeReader(Message) _output_get (Variables|Default|GetmIndex)))

(event EventLookRightAxis
  (params (Axis :type Float%20%28single-precision%29)))

(event EventButtonTop
  ;[1 1 1] Handles the input for the code sequence
  (CallFunction|CheckSequence "Button_Top"))

(event EventMoveButton
  ;[1 1 1] Handles the input for the code sequence
  (CallFunction|CheckSequence "Button_Down"))

(event EventLeftTrigger
  ;[1 1 1] Handles the input for the code sequence
  (CallFunction|CheckSequence "Left_Trigger"))

(event EventRightTrigger
  ;[1 1 1] Handles the input for the code sequence
  (CallFunction|CheckSequence "Right_Trigger"))

(event EventMoveRightAxis
  (params (Axis :type Float%20%28single-precision%29))
  ;[1 1 1] Handles the input for the code sequence
  (if (!= Axis 0.0)
    (if (< Axis 0.0)
      (CallFunction|CheckSequence "Left_Move")
      (else
        (CallFunction|CheckSequence "Right_Move")))))

(fn GenerateSequence
  (Utilities|Array|Clear (Variables|Default|GetmCode_String))
  (Variables|Default|SetmIndex 0)
  (for _index (range 0 (Math|Random|RandomIntegerinRange 1 2))
    (bind _output_get (Variables|Default|Settemp (Utilities|Array|Get(acopy) (Variables|Default|GetmString_Gen) (Math|Random|RandomIntegerinRange 0 (Variables|Default|GetmNum_inputs)))))
    (Utilities|Array|Add (Variables|Default|GetmCode_String) _output_get)
    (Development|PrintString _output_get false)))

(fn CheckSequence
  (params (Input :type String))
  (bind _mindex (Variables|Default|GetmIndex))
  (bind _mindex_2 (Variables|Default|GetmIndex))
  (bind _hud_ref (Variables|Default|GetHUD%20Ref))
  (bind _mcode_string (Variables|Default|GetmCode_String))
  (bind _hud_ref_2 (Variables|Default|GetHUD%20Ref))
  (bind _returnvalue (Utilities|Array|Length _mcode_string))
  (bind _returnvalue_2 (+ _mindex_2 1))
  (bind _returnvalue_3 (< _mindex _returnvalue))
  (if (<= (Variables|Default|GetmInputCooldown) 0.0)
    (if _returnvalue_3
      (if (Utilities|Enum|Equal(Enum) (Utilities|Array|Get(acopy) (Variables|Default|GetmCode_String) _mindex) Input)
        (if _returnvalue_3
          (if (< _returnvalue_2 (Utilities|Array|Length (Variables|Default|GetmCode_String)))
            (Development|PrintString (Utilities|String|Append "Next input is " (Utilities|Array|Get(acopy) (Variables|Default|GetmCode_String) _returnvalue_2)) false))
          (Math|Integer|IncrementInt _mindex
            (:%20%20
              (if (< (Variables|Default|GetmIndex) (Utilities|Array|Length (Variables|Default|GetmCode_String)))
                _
                (else
                  (bind _output_get (Variables|Default|SetmScare_Mult (+ (Variables|Default|GetmScare_Mult) (* (/ 7.0 (Variables|Default|GetmTime_For_Sequence)) 0.5))))
                  (Variables|Default|SetmCan_Scare true)
                  (CallFunction|GenerateSequence)
                  ;[0 0 1] Reset HUD elements
                  (Class|BPIHUDInterface|DestroyCodeReader(Message) _hud_ref)
                  (Class|BPIHUDInterface|MakeCodeReader(Message) _hud_ref (Variables|Default|GetmCode_String))
                  (Development|PrintString (Utilities|String|ToString(Float) _output_get) false)
                  (Variables|Default|SetmTime_For_Sequence 0.0)))
              (CallFunction|AddCooldown :!label _label)
              ;[0 0 1] Update the HUD
              (Class|BPIHUDInterface|UpdateCodeReader(Message) (Variables|Default|GetHUD%20Ref) (Variables|Default|GetmIndex)))))
        (else
          (CallFunction|GenerateSequence)
          ;[0 0 1] Reset HUD elements
          (Class|BPIHUDInterface|DestroyCodeReader(Message) _hud_ref_2)
          (Class|BPIHUDInterface|MakeCodeReader(Message) _hud_ref_2 (Variables|Default|GetmCode_String))
          (Variables|Default|SetmScare_Mult (- (Variables|Default|GetmScare_Mult) 0.5))
          (Class|PossesableComponent|SetStamina (Variables|Default|GetmFailStam) true)
          (goto _label))))))

(fn AddCooldown
  (Variables|Default|SetmInputCooldown 1.5))

(fn SetDefaults
  (Utilities|Array|Clear (Variables|Default|GetmCode_String))
  (Variables|Default|SetmScare_Mult 0.75)
  (Variables|Default|SetmCan_Scare false)
  (Variables|Default|SetInProp false)
  (Variables|Default|SetmTime_For_Sequence 0.0)
  (Variables|Default|SetmInputCooldown 0.0))