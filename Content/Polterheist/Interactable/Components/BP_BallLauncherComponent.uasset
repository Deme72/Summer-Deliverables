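; Interactable component that lets a player possessing a BP_BallLauncher turn it, aim and fire a BP_Ball.
; While controlled, Tick ping-pongs a meter and draws a debug aim arrow.
; The first scare press locks power, the second locks accuracy, where a lower value means less random spread.
; The ball spawns as a sub-pawn, receives power and direction through BP_BallComponent.LaunchingBall, and control ends.
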(event EventTick
  (params (DeltaSeconds :type Float%20%28single-precision%29))
  (bind _launcher_ref (Variables|Default|GetLauncher_ref))
  (bind _launch_spot (Variables|/Game/Polterheist/Interactable/Static/BP_BallLauncher.BP_BallLauncher_C|GetLaunch_spot _launcher_ref))
  ;[1 1 1] Setting UI Vars - DemeFix
  (if (Variables|Default|GetControling)
    (Variables|Default|SetBar (|(b+(dT*d)) (Variables|Default|GetBar) DeltaSeconds (Variables|Default|GetbarDir)))
    (if (>= (Variables|Default|GetBar) 1.0)
      (Variables|Default|SetbarDir -1.0)
      (elif (<= (Variables|Default|GetBar) 0.0)
        (Variables|Default|SetbarDir 1.0)))
    ;[1 1 1] Draws and arrow for the player to know which way they are facing for when they launch a ball
    (Rendering|Debug|DrawDebugArrow (Transformation|GetWorldLocation (Variables|/Game/Polterheist/Interactable/Static/BP_BallLauncher.BP_BallLauncher_C|GetArrow_start _launcher_ref)) (+ (Transformation|GetWorldLocation _launch_spot) (* (Math|Vector|GetForwardVector (Transformation|GetWorldRotation _launch_spot)) (.x (.Max (Components|StaticMesh|GetLocalBounds (Variables|/Script/Polterheist.PossessablePawn|GetStaticMeshComponent _launcher_ref)))))) 3e+02 "(R=0.000000,G=1.000000,B=1.000000,A=1.000000)" 0.0 5.0)
    (else
      (Variables|Default|SetBar 0.0)
      (Variables|Default|SetbarDir 1.0))))

(event EventOnInteract
  (Variables|Default|SetControling true)
  (Variables|Default|SetPowerMode true)
  (Variables|Default|SetAccuracyMode false)
  ;[1 1 1] Gets a reference to the ball launcher this component is attached to
  (bind _aspossessable_pawn (Utilities|Casting|CastToPossessablePawn (Components|GetOwner)))
  (bind _asbp_ball_launcher (Utilities|Casting|CastToBP_BallLauncher _aspossessable_pawn))
  (Variables|Default|SetLauncher_ref _asbp_ball_launcher))

(event EventEndInteract
  (Variables|Default|SetControling false))

(event EventMoveRightAxis
  (params (Axis :type Float%20%28single-precision%29))
  ;[1 1 1] Turns the ball launcherto face a new direction
  (Transformation|AddActorLocalRotation (Variables|Default|GetLauncher_ref) (Math|Rotator|MakeRotator 0.0 0.0 (* Axis (* (Utilities|Time|GetWorldDeltaSeconds) 5.0))) false false))

(event EventScareButton
  ;[1 1 1] Launches a ball
  (CallFunction|LaunchBall))

(fn LaunchBall
  (bind _bar (Variables|Default|GetBar))
  (bind _launcher_ref (Variables|Default|GetLauncher_ref))
  (bind _bar_2 (Variables|Default|GetBar))
  (bind _launch_spot (Variables|/Game/Polterheist/Interactable/Static/BP_BallLauncher.BP_BallLauncher_C|GetLaunch_spot _launcher_ref))
  (bind _returnvalue (Transformation|GetWorldRotation _launch_spot))
  (bind (_roll _pitch _yaw) (Math|Rotator|BreakRotator _returnvalue))
  (if (Variables|Default|GetControling)
    (if (Variables|Default|GetPowerMode)
      ;[1 1 1] If the power bar is visible then when the user hits the scare button they get power based how close they are to that bar
      (if (>= _bar_2 0.98)
        (Variables|Default|SetPower 1.0)
        (else
          (Variables|Default|SetPower _bar_2)))
      (Variables|Default|SetPowerMode false)
      (Variables|Default|SetAccuracyMode true)
      (Variables|Default|SetbarDir -1.0)
      (else
        ;[1 1 1] Gets Accuracy based on how close the player gets the user bar to the accuracy bar
        (if (<= _bar 0.01)
          (Variables|Default|SetAccuracy 0.0)
          (else
            (Variables|Default|SetAccuracy _bar)))
        ;[1 1 1] Spawns the ball based on Launchers foward and accuracy and sends power to function to add force to ball
        (bind _returnvalue_2 (Class|PossessablePawn|SpawnSubPawn (Variables|Default|GetLauncher_ref) "/Game/Polterheist/Interactable/Dynamic/BP_Ball.BP_Ball_C" (Math|Transform|MakeTransform (+ (Transformation|GetWorldLocation _launch_spot) (* (Math|Vector|GetForwardVector (Math|Rotator|MakeRotator (+ _roll (* (Variables|Default|GetAccuracy) (Math|Random|RandomFloatinRange -5e+01 5e+01))) (+ _pitch (* (Variables|Default|GetAccuracy) (Math|Random|RandomFloatinRange -5e+01 5e+01))) (+ _yaw (* (Variables|Default|GetAccuracy) (Math|Random|RandomFloatinRange -5e+01 5e+01))))) (.x (.Max (Components|StaticMesh|GetLocalBounds (Variables|/Script/Polterheist.PossessablePawn|GetStaticMeshComponent _launcher_ref)))))) "0, 0, 0" "1,1,1")))
        (bind _asbp_ball (Utilities|Casting|CastToBP_Ball _returnvalue_2))
        (bind _asbp_ball_component (Utilities|Casting|CastToBP_BallComponent (Variables|/Script/Polterheist.PossessablePawn|GetPossessableComponent _asbp_ball)))
        (Default|LaunchingBall _asbp_ball_component (Variables|Default|GetPower) (Math|Vector|GetForwardVector (Math|Rotator|MakeRotator (+ _roll (* (Variables|Default|GetAccuracy) (Math|Random|RandomFloatinRange -5e+01 5e+01))) (+ _pitch (* (Variables|Default|GetAccuracy) (Math|Random|RandomFloatinRange -5e+01 5e+01))) (+ _yaw (* (Variables|Default|GetAccuracy) (Math|Random|RandomFloatinRange -5e+01 5e+01))))) (- 5e+01 (* (Variables|Default|GetAccuracy) 5e+01)) (Variables|Default|GetLauncher_ref))
        (Variables|Default|SetControling false)))))