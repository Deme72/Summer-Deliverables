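; Possessable component for BP_BalanceProp, a plate-balancing prop the player steers and uses to scare, with strength scaled by plates left.
; Movement builds lean that the look axes adjust and ABP_Balance displays; full lean or wall hits drop BP_Plate actors, and walls bounce the prop.
; Tick drains stamina, recollects overlapping plates after a cooldown, and ejects when plates or stamina run out.
; Scaring or ending interaction resets position, plates and lean.
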(event EventBeginPlay
  ;[1 1 1] Spawns all plates (at the moment the plate spawning is detatched
  (Variables|Default|SetmPlates (Variables|Default|GetmMax_Plates))
  (Variables|Default|SetmDefaultPosition (Transformation|GetActorLocation (Components|GetOwner)))
  (for _index (range 0 (Variables|Default|GetmMax_Plates))
    (Variables|Default|SetmPlateOffset (+ (Variables|Default|GetmPlateOffset) 3.0))
    (bind _asbp_balance_prop (Utilities|Casting|CastToBP_BalanceProp (Components|GetOwner)))
    (Variables|Default|SetmParentRef _asbp_balance_prop)))

(event EventTick
  (params (DeltaSeconds :type Float%20%28single-precision%29))
  (if (Variables|Default|GetInProp)
    ;[1 1 1] Checks if you should still be in prop
    (if (< (Variables|Default|GetmPlates) 1)
      (Class|PossesableComponent|Eject)
      (else
        (bind _returnvalue (Class|PossesableComponent|GetStamina))
        (if (< _returnvalue 1.0)
          (Class|PossesableComponent|Eject)
          (else
            (if (Variables|Default|GetCanMove)
              _
              (else
                (CallFunction|Bouncing)))
            (CallFunction|CapLean)
            (CallFunction|Collide)
            (CallFunction|SetAnimVariables)
            (Class|PossesableComponent|SetStamina -0.005 true)
            (if (Variables|Default|GetmOnCooldown)
              (Variables|Default|SetmPlateLoseTimer (- (Variables|Default|GetmPlateLoseTimer) DeltaSeconds))
              (if (< (Variables|Default|GetmPlateLoseTimer) 0.0)
                (Variables|Default|SetmOnCooldown false)
                (Utilities|Casting|CastToBP_BalanceProp (Components|GetOwner)))
              (else
                (CallFunction|MaybeLosePlate)))))))))

(event EventMoveForwardAxis
  (params (Axis :type Float%20%28single-precision%29))
  ;[1 1 1] Starts to lean in the opposite direction of movement.  leaning 0 is left/right 1 is front /back
  (if (Variables|Default|GetCanMove)
    (bind _sweephitresult (Transformation|AddActorLocalOffset (Components|GetOwner) (Math|Vector|MakeVector (* Axis (Variables|Default|GetmMoveSpeed)) 0.0 0.0) true false))
    (Utilities|Array|SetArrayElem (Variables|Default|GetLeaning) 0 (+ (Utilities|Array|Get(acopy) (Variables|Default|GetLeaning)) (* Axis 0.01)))
    ;[1 1 1] Checks for horizontal collision
    (CallFunction|CollidewithHorizontal? (.Normal (Collision|BreakHitResult _sweephitresult)))))

(event EventMoveRightAxis
  (params (Axis :type Float%20%28single-precision%29))
  ;[1 1 1] Starts to lean in the opposite direction of movement.  leaning 0 is left/right 1 is front /back
  (if (Variables|Default|GetCanMove)
    (bind _sweephitresult (Transformation|AddActorLocalOffset (Components|GetOwner) (Math|Vector|MakeVector 0.0 (* (Variables|Default|GetmMoveSpeed) Axis) 0.0) true false))
    (Utilities|Array|SetArrayElem (Variables|Default|GetLeaning) 1 (+ (Utilities|Array|Get(acopy) (Variables|Default|GetLeaning) 1) (* Axis 0.01)))
    ;[1 1 1] Checks for horizontal collision
    (CallFunction|CollidewithHorizontal? (.Normal (Collision|BreakHitResult _sweephitresult)))))

(event EventLookRightAxis
  (params (Axis :type Float%20%28single-precision%29))
  ;[1 1 1] Right stick correction
  (if (not (== Axis 0.0))
    (Utilities|Array|SetArrayElem (Variables|Default|GetLeaning) 1 (+ (Utilities|Array|Get(acopy) (Variables|Default|GetLeaning) 1) (* Axis -0.002)))))

(event EventLookUpAxis
  (params (Axis :type Float%20%28single-precision%29))
  ;[1 1 1] Right stick correction
  (if (not (== Axis 0.0))
    (Utilities|Array|SetArrayElem (Variables|Default|GetLeaning) 0 (+ (Utilities|Array|Get(acopy) (Variables|Default|GetLeaning)) (* Axis 0.002)))))

(event EventScareButton
  (Class|PossesableComponent|Scare (/ (* (Variables|Default|GetmPlates) 1.0) (Math|Conversions|ToFloat(Integer) (Variables|Default|GetmMax_Plates))))
  (Class|PossesableComponent|SetStamina (Variables|Default|GetmScareStam) true)
  (Class|PossesableComponent|Eject)
  (CallFunction|SetDefaults))

(event EventEndInteract
  (Variables|Default|SetInProp false)
  (CallFunction|SetDefaults))

(event EventOnInteract
  (Variables|Default|SetInProp true))

(fn SetDefaults
  (Transformation|SetActorLocation (Components|GetOwner) (Variables|Default|GetmDefaultPosition) false true)
  (Variables|Default|SetmPlates (Variables|Default|GetmMax_Plates))
  (Variables|Default|SetLeaning (Utilities|Array|MakeArray 0.0 0.0))
  (CallFunction|SetAnimVariables))

(fn SetAnimVariables
  (bind _asabp_balance (Utilities|Casting|CastToABP_Balance (Components|SkeletalMesh|GetAnimInstance (Variables|/Script/Polterheist.PossessablePawn|GetSkeletalMeshComponent (Variables|Default|GetmParentRef)))))
  (Variables|/Game/Polterheist/Interactable/Dynamic/ABP_Balance.ABP_Balance_C|SetHorizontal _asabp_balance (Utilities|Array|Get(acopy) (Variables|Default|GetLeaning)))
  (Variables|/Game/Polterheist/Interactable/Dynamic/ABP_Balance.ABP_Balance_C|SetVertical _asabp_balance (Utilities|Array|Get(acopy) (Variables|Default|GetLeaning) 1)))

(fn MaybeLosePlate
  (bind _leaning (Variables|Default|GetLeaning))
  (bind _leaning_2 (Variables|Default|GetLeaning))
  (bind _output (Utilities|Array|Get(acopy) _leaning_2 1))
  (bind _output_2 (Utilities|Array|Get(acopy) _leaning))
  ;[1 1 1] Check for left/right loss of plate
  (if (or (< _output_2 -0.999) (> _output_2 0.999))
    (CallFunction|LosePlate)
    ;[1 1 1] Check for front/back loss of plate
    (Variables|Default|SetmOnCooldown true)
    (Variables|Default|SetmPlateLoseTimer 2.0)
    (elif (or (< _output -0.999) (> _output 0.999))
      (CallFunction|LosePlate)
      (Variables|Default|SetmOnCooldown true)
      (Variables|Default|SetmPlateLoseTimer 2.0))))

(fn LosePlate
  (bind _mparentref (Variables|Default|GetmParentRef))
  (bind _returnvalue (Transformation|GetActorTransform _mparentref))
  ;[1 1 1] Spawns Plate Pile
  (LocalVariables|SetRanval (Math|Random|RandomIntegerinRange 1 3))
  (Variables|Default|SetmPlates (- (Variables|Default|GetmPlates) (LocalVariables|GetRanval)))
  (for _index (range 1 (LocalVariables|GetRanval))
    (Game|SpawnActorfromClass "/Game/Polterheist/Interactable/Dynamic/BP_Plate.BP_Plate_C" (Math|Transform|MakeTransform (Math|Vector|MakeVector (.x (.location _returnvalue)) (.y (.location _returnvalue)) (- (.z (.location _returnvalue)) (- 9e+01 (Math|Conversions|ToFloat(Integer) (* _index 3))))) (.rotation _returnvalue) (.scale _returnvalue)) "AlwaysSpawn" 0 0))
  (Development|PrintString (Utilities|String|ToString(Integer) (Variables|Default|GetmPlates)))
  (Class|PossesableComponent|SetStamina -1e+01 true))

(fn Collide
  (if (< (Variables|Default|GetmPlateLoseTimer) 0.0)
    (bind (_outactors _returnvalue) (Collision|CapsuleOverlapActors (Transformation|GetActorLocation (Components|GetOwner)) 35.0 1e+02 (Utilities|Array|MakeArray "ObjectTypeQuery2") "/Game/Polterheist/Interactable/Dynamic/BP_Plate.BP_Plate_C"))
    (if _returnvalue
      (for _array_element _outactors
        (bind _output_get (Variables|Default|SetmPlates (+ (Variables|Default|GetmPlates) 1)))
        (Actor|DestroyActor _array_element)
        (Development|PrintString (Utilities|String|ToString(Integer) _output_get))))))

(fn CollidewithHorizontal?
  (params (Normal :type Vector))
  (if (or (or (Math|Vector|Equal(Vector) Normal "0,1.000000, 0" 0.001) (Math|Vector|Equal(Vector) Normal "1.000000, 0, 0" 0.001)) (or (Math|Vector|Equal(Vector) Normal "0,-1.000000, 0" 0.001) (Math|Vector|Equal(Vector) Normal "-1.000000, 0, 0" 0.001)))
    (Variables|Default|SetCanMove false)
    (Variables|Default|SetBounceNorm Normal)
    (Variables|Default|SetTimePassed 0.0)
    (CallFunction|LosePlate)))

(fn CapLean
  ;[1 1 1] Caps leaning for use in animations. Should be between -1 and 1
  (for (_array_element _array_index) (Variables|Default|GetLeaning)
    (if (> _array_element 1.0)
      (Utilities|Array|SetArrayElem (Variables|Default|GetLeaning) _array_index 1.0)
      (elif (< _array_element -1.0)
        (Utilities|Array|SetArrayElem (Variables|Default|GetLeaning) _array_index -1.0)))))

(fn Bouncing
  (if (> (Variables|Default|GetTimePassed) 0.5)
    (Variables|Default|SetCanMove true)
    (else
      (Transformation|AddActorLocalOffset (Components|GetOwner) (* (Variables|Default|GetBounceNorm) (Variables|Default|GetBounceAmount)) false false)
      (Variables|Default|SetTimePassed (+ (Variables|Default|GetTimePassed) (Utilities|Time|GetWorldDeltaSeconds))))))