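; BP_ParanoiaBase is an interactable component that makes its owning actor jitter and emit paranoia particles while in use.
; BeginPlay caches the owner's starting rotation as the shake's center.
; Tick uses a short Delay to throttle jumps to small random rotations around that center, each spawning ParanoiaParticle just above the owner.
; When not in use, Tick restores the cached rotation every frame.
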(event EventBeginPlay
  (bind _returnvalue (Components|GetOwner))
  (bind _returnvalue_2 (Transformation|GetActorRotation _returnvalue))
  (bind (_roll _pitch _yaw) (Math|Rotator|BreakRotator _returnvalue_2))
  (Variables|Default|Setx _roll)
  (Variables|Default|Sety _pitch)
  (Variables|Default|Setz _yaw))

(event EventTick
  (params (DeltaSeconds :type Float%20%28single-precision%29))
  (bind _returnvalue (Components|GetOwner))
  (bind _x (Variables|Default|Getx))
  (bind _y (Variables|Default|Gety))
  (bind _z (Variables|Default|Getz))
  (if (Class|InteractableComponent|IsinUse)
    (Utilities|FlowControl|Delay 0.1)
    (Transformation|SetActorRotation _returnvalue (Math|Rotator|Lerp(Rotator) (Transformation|GetActorRotation _returnvalue) (Math|Rotator|MakeRotator (+ _x (Math|Random|RandomFloatinRange -5.0 5.0)) (+ _y (Math|Random|RandomFloatinRange -5.0 5.0)) (+ _z (Math|Random|RandomFloatinRange -5.0 5.0))) 1.0 true))
    (Effects|SpawnEmitteratLocation "/Game/Assets/ParanoiaParticle.ParanoiaParticle" (+ (Transformation|GetActorLocation _returnvalue) "0.000000,0.000000,50.000000"))
    (else
      (Transformation|SetActorRotation _returnvalue (Math|Rotator|MakeRotator _x _y _z)))))