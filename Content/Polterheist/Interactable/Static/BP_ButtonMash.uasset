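; BP_ButtonMash is a static Polterheist interactable that ejects through its ButtonMashComponent a set time after a scare.
; DidScare starts a countdown by setting CurTimer to AnimTime.
; Tick decrements the timer and, when it runs out, looks up the ButtonMashComponent and calls Eject once.
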(event EventBeginPlay)

(event Collision|EventActorBeginOverlap
  (params (OtherActor :type Actor%20Object%20Reference)))

(event EventTick
  (params (DeltaSeconds :type Float%20%28single-precision%29))
  (if (> (Variables|Default|GetcurTimer) 0.0)
    (Variables|Default|SetcurTimer (- (Variables|Default|GetcurTimer) DeltaSeconds))
    (if (not (> (Variables|Default|GetcurTimer) 0.0))
      (Class|PossesableComponent|Eject (Actor|GetComponentbyClass "/Game/Polterheist/Interactable/Components/ButtonMashComponent.ButtonMashComponent_C")))))

(fn ConstructionScript)

(fn DidScare
  (Variables|Default|SetcurTimer (Variables|Default|GetanimTime)))