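; Prototype construction-script builder that assembles millwork from up to four wall mesh pieces, A through D.
; For each wall, a toggle either keeps its static mesh component or destroys it.
; Kept components take their mesh from that wall's own selection list by a per-wall index.
; All logic runs in the Construction Script, and the event graph holds only disabled stub events.
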(event EventBeginPlay)

(event Collision|EventActorBeginOverlap
  (params (OtherActor :type Actor%20Object%20Reference)))

(event EventTick
  (params (DeltaSeconds :type Float%20%28single-precision%29)))

(fn ConstructionScript
  (bind _sm_cl_solidwall_a1 (Variables|Default|GetSM_CL_SolidWall_A1))
  (bind _sm_cl_solidwall_a2 (Variables|Default|GetSM_CL_SolidWall_A2))
  (bind _sm_cl_solidwall_a3 (Variables|Default|GetSM_CL_SolidWall_A3))
  (bind _sm_cl_solidwall_a4 (Variables|Default|GetSM_CL_SolidWall_A4))
  (Utilities|FlowControl|Sequence
    (:then_0
      (if (Variables|Default|GetWall%20A)
        (Components|StaticMesh|SetStaticMesh _sm_cl_solidwall_a1 (Utilities|Array|Get(acopy) (Variables|Default|GetWall_A_Select) (Variables|Default|Getv_Wall_A_Select)))
        (else
          (Components|DestroyComponent _sm_cl_solidwall_a1))))
    (:then_1
      (if (Variables|Default|GetWall%20B)
        (Components|StaticMesh|SetStaticMesh _sm_cl_solidwall_a2 (Utilities|Array|Get(acopy) (Variables|Default|GetWall_B_Select) (Variables|Default|Getv_Wall_B_Select)))
        (else
          (Components|DestroyComponent _sm_cl_solidwall_a2))))
    (:then_2
      (if (Variables|Default|GetWall%20C)
        (Components|StaticMesh|SetStaticMesh _sm_cl_solidwall_a3 (Utilities|Array|Get(acopy) (Variables|Default|GetWall_C_Select) (Variables|Default|Getv_Wall_C_Select)))
        (else
          (Components|DestroyComponent _sm_cl_solidwall_a3))))
    (:then_3
      (if (Variables|Default|GetWall%20D)
        (Components|StaticMesh|SetStaticMesh _sm_cl_solidwall_a4 (Utilities|Array|Get(acopy) (Variables|Default|GetWall_D_Select) (Variables|Default|Getv_Wall_D_Select)))
        (else
          (Components|DestroyComponent _sm_cl_solidwall_a4))))))