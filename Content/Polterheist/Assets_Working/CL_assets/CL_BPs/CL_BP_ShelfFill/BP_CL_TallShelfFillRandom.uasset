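; Tall shelf actor that fills five slots with varied shelf-fill Blueprints through Child Actor components.
; The construction script sets each component's class from the BPShelfFill array using its own stored index.
; Turning on Randomize rerolls all five indices, then clears itself, so it acts as an editor button and the layout holds on later reconstruction.
; The Event Graph has no active logic.
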(event EventBeginPlay)

(event Collision|EventActorBeginOverlap
  (params (OtherActor :type Actor%20Object%20Reference)))

(event EventTick
  (params (DeltaSeconds :type Float%20%28single-precision%29)))

(fn ConstructionScript
  (if (Variables|Default|GetRandomize)
    (Variables|Default|SetvBP_ShelfFill (Math|Random|RandomIntegerinRange 0 4))
    (Variables|Default|SetvBP_ShelfFill_0 (Math|Random|RandomIntegerinRange 0 4))
    (Variables|Default|SetvBP_ShelfFill_1 (Math|Random|RandomIntegerinRange 0 4))
    (Variables|Default|SetvBP_ShelfFill_2 (Math|Random|RandomIntegerinRange 0 4))
    (Variables|Default|SetvBP_ShelfFill_3 (Math|Random|RandomIntegerinRange 0 4))
    (Variables|Default|SetRandomize false))
  (ChildActorComponent|SetChildActorClass (Variables|Default|GetBP_CL_ShelfFillRandom) (Utilities|Array|Get(acopy) (Variables|Default|GetBP_ShelfFill) (Variables|Default|GetvBP_ShelfFill)))
  (ChildActorComponent|SetChildActorClass (Variables|Default|GetBP_CL_ShelfFillRandom1) (Utilities|Array|Get(acopy) (Variables|Default|GetBP_ShelfFill) (Variables|Default|GetvBP_ShelfFill_0)))
  (ChildActorComponent|SetChildActorClass (Variables|Default|GetBP_CL_ShelfFillRandom2) (Utilities|Array|Get(acopy) (Variables|Default|GetBP_ShelfFill) (Variables|Default|GetvBP_ShelfFill_1)))
  (ChildActorComponent|SetChildActorClass (Variables|Default|GetBP_CL_ShelfFillRandom3) (Utilities|Array|Get(acopy) (Variables|Default|GetBP_ShelfFill) (Variables|Default|GetvBP_ShelfFill_2)))
  (ChildActorComponent|SetChildActorClass (Variables|Default|GetBP_CL_ShelfFillRandom4) (Utilities|Array|Get(acopy) (Variables|Default|GetBP_ShelfFill) (Variables|Default|GetvBP_ShelfFill_3))))