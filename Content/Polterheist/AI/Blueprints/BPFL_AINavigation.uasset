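; Blueprint function library of AI navigation helpers for moving agents through a network of NavigationNodes.
; Blackboard helpers read and write the previous node, next node and target position through key selectors.
; Advance shifts the by-ref node pair forward to a random neighbor from the NavNetManager; AdvancePoi prefers a POI neighbor and falls back to Advance.
; GetRandomPositionAroundNode projects a random offset within a radius onto the navmesh.
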(fn GetBlackboardNodes
  (params (BlackboardRef :type Blackboard%20Component%20Object%20Reference) (PreviousNodeKey :type Blackboard%20Key%20Selector%20Structure) (NextNodeKey :type Blackboard%20Key%20Selector%20Structure))
  (Utilities|FlowControl|Sequence
    (:then_0
      ;[1 1 1] Get blackboard 'Previous Node'
      (bind _asnavigation_node (Utilities|Casting|CastToNavigationNode (AI|Components|Blackboard|GetValueasObject BlackboardRef (.SelectedKeyName (Utilities|Struct|BreakBlackboardKeySelector PreviousNodeKey))))
        (:CastFailed
          (Development|PrintString 0 "Cast to Navigation Node failed" true true "(R=1.000000,G=0.000000,B=0.000000,A=1.000000)" :!label _label))))
    (:then_1
      ;[1 1 1] Get blackboard 'Next Node'
      (bind _asnavigation_node_2 (Utilities|Casting|CastToNavigationNode (AI|Components|Blackboard|GetValueasObject BlackboardRef (.SelectedKeyName (Utilities|Struct|BreakBlackboardKeySelector NextNodeKey))))
        (:CastFailed
          (goto _label))))
    (:then_2
      _))
  (return _asnavigation_node _asnavigation_node_2))

(fn SetBlackboardNodes
  (params (BlackboardRef :type Blackboard%20Component%20Object%20Reference) (PreviousNodeKey :type Blackboard%20Key%20Selector%20Structure) (NextNodeKey :type Blackboard%20Key%20Selector%20Structure) (NewPreviousNode :type Navigation%20Node%20Object%20Reference) (NewNextNode :type Navigation%20Node%20Object%20Reference))
  (AI|Components|Blackboard|SetValueasObject BlackboardRef (.SelectedKeyName (Utilities|Struct|BreakBlackboardKeySelector PreviousNodeKey)) NewPreviousNode)
  (AI|Components|Blackboard|SetValueasObject BlackboardRef (.SelectedKeyName (Utilities|Struct|BreakBlackboardKeySelector NextNodeKey)) NewNextNode)
  (return))

(fn SetAllBlackboardValues
  (params (BlackboardRef :type Blackboard%20Component%20Object%20Reference) (PreviousNodeKey :type Blackboard%20Key%20Selector%20Structure) (NextNodeKey :type Blackboard%20Key%20Selector%20Structure) (TargetPositionKey :type Blackboard%20Key%20Selector%20Structure) (NewPreviousNode :type Navigation%20Node%20Object%20Reference) (NewNextNode :type Navigation%20Node%20Object%20Reference) (NewTargetPosition :type Vector))
  (Utilities|FlowControl|Sequence
    (:then_0
      ;[1 1 1] Set blackboard 'PreviousPoint' to 'NewPreviousNode'
      (AI|Components|Blackboard|SetValueasObject BlackboardRef (.SelectedKeyName (Utilities|Struct|BreakBlackboardKeySelector PreviousNodeKey)) NewPreviousNode))
    (:then_1
      ;[1 1 1] Set blackboard 'TargetPoint' to 'NewTargetNode'
      (AI|Components|Blackboard|SetValueasObject BlackboardRef (.SelectedKeyName (Utilities|Struct|BreakBlackboardKeySelector NextNodeKey)) NewNextNode))
    (:then_2
      ;[1 1 1] Set blackboard 'TargetPos' to 'NewTargetPos'
      (AI|Components|Blackboard|SetValueasVector BlackboardRef (.SelectedKeyName (Utilities|Struct|BreakBlackboardKeySelector TargetPositionKey)) NewTargetPosition))
    (:then_3
      (return))))

(fn GetRandomNeighborNode
  (params (NavNetManagerRef :type BP%20Nav%20Net%20Manager%20Object%20Reference%20%28by%20ref%29) (PreviousNode :type Navigation%20Node%20Object%20Reference%20%28by%20ref%29) (NextNode :type Navigation%20Node%20Object%20Reference%20%28by%20ref%29))
  (bind (_isnew _returnvalue) (Class|NavigationNetworkManager|GetNodeNeighbors NavNetManagerRef PreviousNode NextNode))
  (return (Utilities|Array|Get(acopy) _returnvalue (Math|Random|RandomIntegerinRange 0 (Utilities|Array|LastIndex _returnvalue))) _isnew))

(fn GetRandomNeighborPoi
  (params (NavNetManagerRef :type BP%20Nav%20Net%20Manager%20Object%20Reference) (PreviousNode :type Navigation%20Node%20Object%20Reference) (NextNode :type Navigation%20Node%20Object%20Reference))
  (bind (_haspoi _returnvalue) (Class|NavigationNetworkManager|GetPoiNeighbors NavNetManagerRef NextNode PreviousNode))
  (return (Utilities|Array|Get(acopy) _returnvalue (Math|Random|RandomIntegerinRange 0 (Utilities|Array|LastIndex _returnvalue))) _haspoi))

(fn GetRandomPositionAroundNode
  (params (Node :type Navigation%20Node%20Object%20Reference) (Max%20Radius :type Float%20%28single-precision%29))
  (bind _returnvalue (Math|Random|RandomFloatinRange 1.0 3.6e+02))
  (bind _returnvalue_2 (Math|Random|RandomFloatinRange 1.0 Max%20Radius))
  (bind _returnvalue_3 (Transformation|GetActorLocation Node))
  (bind _returnvalue_4 (Math|Vector|MakeVector 1.0 0.0 0.0))
  (bind _returnvalue_5 (Math|Rotator|MakeRotator 0.0 0.0 _returnvalue))
  (bind _returnvalue_6 (Math|Vector|RotateVector _returnvalue_4 _returnvalue_5))
  (bind _returnvalue_7 (* _returnvalue_6 _returnvalue_2))
  (bind _returnvalue_8 (+ _returnvalue_3 _returnvalue_7))
  (bind (_projectedlocation _returnvalue_9) (AI|Navigation|ProjectPointtoNavigation 0 _returnvalue_8 0 0))
  (return _projectedlocation _returnvalue_9))

(fn Advance
  (params (NavNetManagerRef :type BP%20Nav%20Net%20Manager%20Object%20Reference) (TempPreviousNode :type Navigation%20Node%20Object%20Reference%20%28by%20ref%29) (TempNextNode :type Navigation%20Node%20Object%20Reference%20%28by%20ref%29))
  (bind (_neighbornode _isnewnode) (CallFunction|GetRandomNeighborNode NavNetManagerRef TempPreviousNode TempNextNode))
  (|SetBy-RefVar TempPreviousNode TempNextNode)
  (|SetBy-RefVar TempNextNode _neighbornode)
  (return (not _isnewnode)))

(fn AdvancePoi
  (params (NavNetManagerRef :type BP%20Nav%20Net%20Manager%20Object%20Reference) (TempPreviousNode :type Navigation%20Node%20Object%20Reference) (TempNextNode :type Navigation%20Node%20Object%20Reference))
  (bind (_poi_neighbor _success) (CallFunction|GetRandomNeighborPoi NavNetManagerRef TempPreviousNode TempNextNode))
  (if _success
    (|SetBy-RefVar TempPreviousNode TempNextNode)
    (|SetBy-RefVar TempNextNode _poi_neighbor)
    (else
      (CallFunction|Advance NavNetManagerRef TempPreviousNode TempNextNode)))
  (return _success))