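; Possessable painting pawn that lets a player look out through a network of linked paintings.
; Possession eases the camera onto the painting, and A/D or arrow keys cycle the network, swapping in each painting's render material.
; The selected painting shows tinted eyes, and a post-process material overlays its view frame.
; Left Shift moves the camera to the ThirdPersonCharacter's view and repossesses that character.
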(event EventBeginPlay
  (bind _is_oval (Variables|Default|GetIs_Oval))
  (CallFunction|ChangeViewFrame (Variables|Default|GetGREEEN))
  (CallFunction|SetDeafaultPaint)
  (Variables|Default|SetArrayPos (Variables|Default|GetArrayStart))
  (CallFunction|ToggleEyes false)
  (CallFunction|SetNetwork)
  (Development|SetHiddeninGame (Variables|Default|GetFrame) _is_oval false)
  (Development|SetHiddeninGame (Variables|Default|GetOval_Frame) (not _is_oval) false))

(event Collision|EventActorBeginOverlap
  (params (OtherActor :type Actor%20Object%20Reference)))

(event EventTick
  (params (DeltaSeconds :type Float%20%28single-precision%29)))

(event EventUnpossessed
  (params (OldController :type Controller%20Object%20Reference))
  (CallFunction|ToggleEyes (Utilities|ResolveSoftReference (Utilities|Array|Get(acopy) (Variables|Default|GetPaintingsNetwork) (Variables|Default|GetArrayPos))) false)
  (CallFunction|SetDeafaultPaint)
  (Development|SetHiddeninGame (Variables|Default|GetPainting) true false))

(event EventPossessed
  (params (NewController :type Controller%20Object%20Reference))
  (bind _cube (Variables|Default|GetCube))
  (bind _returnvalue (Transformation|GetRelativeTransform _cube))
  (CallFunction|ChangeViewFrame (Variables|Default|GetGREEEN))
  (Development|SetHiddeninGame (Variables|Default|GetPainting) false false)
  (Variables|Default|SetArrayPos (Variables|Default|GetArrayStart))
  (Variables|Default|SetMoveEye false)
  (Rendering|Material|SetMaterial (Variables|Default|GetPainting1) 0 (Variables|Default|GetRipple))
  (Components|MoveComponentTo (Variables|Default|GetViewCamera) (.location _returnvalue) (.rotation _returnvalue) false false 0.4 false)
  (CallFunction|SetDeafaultPaint)
  (CallFunction|SettoCams)
  (CallFunction|ChangeViewFrame (Variables|Default|GetGREEEN))
  (CallFunction|ChangeViewFrame (Variables|Default|GetViewFrame?)))

(event Input|KeyboardEvents|LeftShift
  (params (Key :type Key%20Structure :default "None"))
  (bind _revert_cube (Variables|Default|GetRevert%20Cube))
  (bind _returnvalue (Transformation|GetRelativeTransform _revert_cube))
  (:Pressed
    (CallFunction|ChangeViewFrame (Variables|Default|GetGREEEN))
    (bind _outactors (Actor|GetAllActorsOfClass "/Game/ThirdPersonBP/Blueprints/ThirdPersonCharacter.ThirdPersonCharacter_C"))
    (Variables|Default|SetMoveEye true)
    (Transformation|SetWorldTransform _revert_cube (Math|Transform|MakeTransform (.location (Transformation|GetWorldTransform (Variables|/Game/ThirdPersonBP/Blueprints/ThirdPersonCharacter.ThirdPersonCharacter_C|GetFollowCamera (Utilities|Array|Get(acopy) _outactors)))) (.rotation (Transformation|GetWorldTransform (Variables|/Game/ThirdPersonBP/Blueprints/ThirdPersonCharacter.ThirdPersonCharacter_C|GetFollowCamera (Utilities|Array|Get(acopy) _outactors)))) "1,1,1") false false)
    (CallFunction|SetDeafaultPaint)
    (Components|MoveComponentTo (Variables|Default|GetViewCamera) (.location _returnvalue) (.rotation _returnvalue) false false 0.2 false)
    (Pawn|Possess (Pawn|GetController) (Utilities|Array|Get(acopy) _outactors))))

(event Input|KeyboardEvents|Left
  (params (Key :type Key%20Structure :default "None"))
  (:Pressed
    (CallFunction|ChangeCam -1)))

(event Input|KeyboardEvents|Right
  (params (Key :type Key%20Structure :default "None"))
  (:Pressed
    (CallFunction|ChangeCam 1)))

(event Input|KeyboardEvents|A
  (params (Key :type Key%20Structure :default "None"))
  (:Pressed
    (CallFunction|ChangeCam -1)))

(event Input|KeyboardEvents|D
  (params (Key :type Key%20Structure :default "None"))
  (:Pressed
    (CallFunction|ChangeCam 1)))

(fn ConstructionScript)

(fn SetDeafaultPaint
  (Rendering|Material|SetMaterial (Variables|Default|GetPainting) 0 (Variables|Default|GetDefault%20Painting)))

(fn SettoCams
  (bind _painting (Variables|Default|GetPainting))
  (bind _arraypos (Variables|Default|GetArrayPos))
  (bind _paintingsnetwork (Variables|Default|GetPaintingsNetwork))
  (bind _output (Utilities|Array|Get(acopy) _paintingsnetwork _arraypos))
  (if (== (Utilities|ResolveSoftReference _output) 0)
    (Rendering|Material|SetMaterial _painting 0 (Variables|Default|GetRenderMat))
    (else
      (Rendering|Material|SetMaterial _painting 0 (Variables|Painting_C|GetRenderMat (Utilities|ResolveSoftReference _output))))))

(fn ChangeCam
  (params (Dir :type Integer))
  (bind _paintingsnetwork (Variables|Default|GetPaintingsNetwork))
  (bind _returnvalue (Utilities|Array|Length _paintingsnetwork))
  (CallFunction|ToggleEyes (Utilities|ResolveSoftReference (Utilities|Array|Get(acopy) (Variables|Default|GetPaintingsNetwork) (Variables|Default|GetArrayPos))) false)
  (if (>= (+ (Variables|Default|GetArrayPos) Dir) _returnvalue)
    (Variables|Default|SetArrayPos 0)
    (elif (< (+ (Variables|Default|GetArrayPos) Dir) 0)
      (Variables|Default|SetArrayPos (- _returnvalue 1))
      (else
        (Variables|Default|SetArrayPos (+ (Variables|Default|GetArrayPos) Dir)))))
  (Rendering|Material|SetMaterial (Variables|Default|GetPainting) 0 (Variables|Painting_C|GetRenderMat (Utilities|ResolveSoftReference (Utilities|Array|Get(acopy) (Variables|Default|GetPaintingsNetwork) (Variables|Default|GetArrayPos)))))
  (CallFunction|SetEyeCol (Utilities|ResolveSoftReference (Utilities|Array|Get(acopy) (Variables|Default|GetPaintingsNetwork) (Variables|Default|GetArrayPos))) (Variables|Default|GetEyeCol))
  (CallFunction|ToggleEyes (Utilities|ResolveSoftReference (Utilities|Array|Get(acopy) (Variables|Default|GetPaintingsNetwork) (Variables|Default|GetArrayPos))) true)
  (CallFunction|ChangeViewFrame (Variables|Painting_C|GetViewFrame? (Utilities|ResolveSoftReference (Utilities|Array|Get(acopy) (Variables|Default|GetPaintingsNetwork) (Variables|Default|GetArrayPos))))))

(fn PossessCam
  (params (Camera :type Camera%20Component%20Object%20Reference))
  (bind _returnvalue (Transformation|GetWorldTransform Camera))
  (Transformation|SetWorldTransform (Variables|Default|GetViewCamera) (Math|Transform|MakeTransform (.location _returnvalue) (.rotation _returnvalue) "1,1,1") false false))

(fn SetNetwork
  (if (== (Variables|Default|GetPaintingNetwork) 1)
    (Variables|Default|SetPaintingsNetwork (Variables|Default|GetPaintings_1))
    (elif (== (Variables|Default|GetPaintingNetwork) 2)
      (Variables|Default|SetPaintingsNetwork (Variables|Default|GetPaintings_2)))))

(fn ToggleEyes
  (params (Activate :type Boolean))
  (bind _lefteye_follow (Variables|Default|GetLeftEye_Follow))
  (if Activate
    (Development|SetHiddeninGame _lefteye_follow false true)
    (Variables|Default|SetMoveEye true)
    (else
      (Development|SetHiddeninGame _lefteye_follow true true)
      (Variables|Default|SetMoveEye false))))

(fn GhostInside
  (return (Variables|Default|GetMoveEye)))

(fn ChangeViewFrame
  (params (Texture :type Texture%20Object%20Reference))
  (bind _returnvalue (Rendering|Material|CreateDynamicMaterialInstance "/Game/Paintings/ViewCover_A.ViewCover_A" "None" :!class /Script/Engine.KismetMaterialLibrary))
  (Rendering|Material|SetVectorParameterValue _returnvalue "KeyCol" "(R=0.000000,G=1.000000,B=0.000000,A=1.000000)" :!class /Script/Engine.MaterialInstanceDynamic)
  (Rendering|Material|SetTextureParameterValue _returnvalue "FrameTex" Texture)
  (Rendering|Material|SetScalarParameterValue _returnvalue "buffer" 0.55 :!class /Script/Engine.MaterialInstanceDynamic)
  (Utilities|Struct|SetmembersinPostProcessSettings (Variables|/Script/Engine.CameraComponent|GetPostProcessSettings (Variables|Default|GetViewCamera)) (Utilities|Struct|MakeWeightedBlendables (Utilities|Array|MakeArray (Utilities|Struct|MakeWeightedBlendable 1.0 _returnvalue)))))

(fn SetEyeCol
  (params (NewCol :type Color%20Structure))
  (bind _returnvalue (Rendering|Material|CreateDynamicMaterialInstance "/Game/Paintings/TempCols/EyeBall_Inst.EyeBall_Inst" "None" :!class /Script/Engine.KismetMaterialLibrary))
  (Rendering|Material|SetVectorParameterValue _returnvalue "Color" (Math|Conversions|ToLinearColor(Color) NewCol) :!class /Script/Engine.MaterialInstanceDynamic)
  (Rendering|Material|SetMaterial (Variables|Default|GetSphere1) 0 _returnvalue))

(fn PossessSetEyeCol
  (params (NewCol :type Color%20Structure))
  (Variables|Default|SetEyeCol NewCol))